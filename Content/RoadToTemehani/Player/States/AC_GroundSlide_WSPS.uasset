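; Player state component for a ground slide that propels the character along its facing direction, with looping flipbook, sound and Niagara effect.
; IsAccessible steps downward traces ahead to cap the distance before a ledge, allowing the slide only if it is above zero.
; Enter starts a smooth movement; when it finishes, crouch input or lack of headroom selects crouch locomotion, and exiting to any other state uncrouches.
; Per-update wall and void checks exist but are disconnected.
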(fn `Enter`
  (params (PreviousState :type "/Game/RoadToTemehani/Core/StateManager/EPlayerStates Enum" :default "NewEnumerator7"))
  (bind _distance (`self.Distance`))
  (bind _player_actor (`self.Player Actor`))
  (`parent.Enter` PreviousState)
  (add `/Game/RoadToTemehani/Player/BP_Player.OnSmoothMovementFinished` (`self.Player Actor`) (`|CreateDelegate` :!event `OnSmoothMovementFinished`))
  (`/Game/RoadToTemehani/Player/BP_Player.TriggerSmoothMovement` _player_actor (* (`Actor.GetActorForwardVector` _player_actor) _distance) (/ _distance (`self.Speed`)) "NewEnumerator0") ; We propel the player sliding, in the direction that he currently faces.
  (`/Game/RoadToTemehani/Core/FlipbookManager/AC_FlipbookManager.PlayLoopingAnimation` (`self.GetPlayerFlipbookManager`) (`self.GroundSlideFB`) "None")
  (`GameplayStatics.SpawnSound2D` (`self.GroundSlideSFX`) 1.0 1.0 0.0 null)
  (`NiagaraFunctionLibrary.SpawnSystemAttached` (`self.GroundSlideVFX`) (`Character.CapsuleComponent` (`self.Player Actor`)) "None" (0.0 0.0 0.0) (struct) "KeepRelativeOffset")
  (return))

(fn `Exit`
  (params (NextState :type "/Game/RoadToTemehani/Core/StateManager/EPlayerStates Enum" :default "NewEnumerator7"))
  (`parent.Exit` NextState)
  (remove `/Game/RoadToTemehani/Player/BP_Player.OnSmoothMovementFinished` (`self.Player Actor`) (`|CreateDelegate` :!event `OnSmoothMovementFinished`))
  (if (`|EnumInequality` NextState "NewEnumerator6")
    ;[1 1 1] If we stand back up, we uncrouch, with the function uncrouch of the crouch locomotion state. This will resize the hurtbox and allow us to run at full speed
    (bind _stateactorcomponent (`/Game/RoadToTemehani/Core/StateManager/AC_PlayerStatesManager.GetStateActorComponent` (`self.GetPlayerStatesManager`) "NewEnumerator6"))
    (bind _ascrouch_locomotion_state (cast `/Game/RoadToTemehani/Player/States/AC_CrouchLocomotion_PS` _stateactorcomponent))
    (`/Game/RoadToTemehani/Player/States/AC_CrouchLocomotion_PS.Toggle Crouch` _ascrouch_locomotion_state false))
  (return))

(fn `FindMaxSlideDistance`
  (params (SearchPrecision :type "Float (double-precision)" :default 5.0))
  (returns (MaxSlideDistance :type "Float (double-precision)"))
  (locals (L_DistanceToSearch :type "Float (double-precision)") (L_NbSteps :type Integer))
  (bind _player_actor (`self.Player Actor`))
  (bind _returnvalue (+ (`Actor.K2_GetActorLocation` _player_actor) (* (`Actor.GetActorForwardVector` _player_actor) (`local.L_DistanceToSearch`))))
  (bind _output_get (set `local.L_NbSteps` (`KismetMathLibrary.FTrunc` (/ (`self.SlideDistance`) SearchPrecision))))
  (for _index (range (+ _output_get 1))
    (set `local.L_DistanceToSearch` (* _index SearchPrecision))
    (bind (_outhit _returnvalue_2) (`KismetSystemLibrary.LineTraceSingleByProfile` _returnvalue (- _returnvalue (`KismetMathLibrary.MakeVector` 0.0 0.0 (+ (`CapsuleComponent.GetScaledCapsuleHalfHeight` (`Character.CapsuleComponent` _player_actor)) 10.0))) "Pawn"))
    (if (not _returnvalue_2)
      (set `local.L_DistanceToSearch` (- (`local.L_DistanceToSearch`) SearchPrecision (`CapsuleComponent.GetScaledCapsuleRadius` (`Character.CapsuleComponent` (`self.Player Actor`)))))
      (break)))
  (return (`local.L_DistanceToSearch`)))

(fn `FindVoid`
  (returns (OutHit :type "HitResult Structure") (ReturnValue :type Boolean))
  (bind _player_actor (`self.Player Actor`))
  (bind _returnvalue_x (`KismetMathLibrary.BreakVector` (`Actor.GetActorForwardVector` _player_actor)))
  (bind _capsulecomponent (`Character.CapsuleComponent` _player_actor))
  (bind _returnvalue (+ (`Actor.K2_GetActorLocation` _player_actor) (`KismetMathLibrary.MakeVector` (`CapsuleComponent.CapsuleRadius` _capsulecomponent) 0.0 (* (`CapsuleComponent.CapsuleHalfHeight` _capsulecomponent) -1.0))))
  (`KismetSystemLibrary.LineTraceSingle` :`Start` _returnvalue :`End` (+ _returnvalue (* (`KismetMathLibrary.MakeVector` (* (.x (`KismetMathLibrary.GetForwardVector` (`KismetMathLibrary.MakeRotator` 0.0 -50.0))) _returnvalue_x) (.y (`KismetMathLibrary.GetForwardVector` (`KismetMathLibrary.MakeRotator` 0.0 -50.0))) (.z (`KismetMathLibrary.GetForwardVector` (`KismetMathLibrary.MakeRotator` 0.0 -50.0)))) (`self.DiagonalLength`))) :`TraceChannel` "TraceTypeQuery1" :`DrawDebugType` "ForDuration")
  (return (struct) false))

(fn `FindVoidAndWall`
  (returns (FoundObstacle :type Boolean))
  (bind (_outhit _returnvalue) (`self.FindWall`))
  (bind (_outhit_2 _returnvalue_2) (`self.FindVoid`))
  (return _returnvalue))

(fn `FindWall`
  (returns (OutHit :type "HitResult Structure") (ReturnValue :type Boolean))
  (bind _player_actor (`self.Player Actor`))
  (bind _returnvalue (`Actor.K2_GetActorLocation` _player_actor))
  (bind _returnvalue_x (`KismetMathLibrary.BreakVector` (`Actor.GetActorForwardVector` _player_actor)))
  (bind (_outhit _returnvalue_2) (`KismetSystemLibrary.LineTraceSingleForObjects` _returnvalue (+ _returnvalue (`KismetMathLibrary.MakeVector` (* _returnvalue_x (+ (`CapsuleComponent.CapsuleRadius` (`Character.CapsuleComponent` _player_actor)) (`self.WallSearchDistance`))))) (`|MakeArray` "ObjectTypeQuery1" :!type "EObjectTypeQuery Enum") false (`|MakeArray` (`self.Player Actor`) :!type "Actor Object Reference") "ForDuration"))
  (return _outhit _returnvalue_2))

(fn `IsAccessible`
  (returns (bResult :type Boolean))
  ;[1 1 1] We do a ground slide only if the distance to go through is above 0
  (`parent.IsAccessible`)
  (bind _maxslidedistance (`self.FindMaxSlideDistance` 5.0))
  (bind _output_get (set `self.Distance` _maxslidedistance))
  (return (> _output_get 0.0)))

(fn `OnSmoothMovementFinished`
  (bind _states_manager (`self.GetPlayerStatesManager`))
  ;[1 1 1] In order to reach the ground locomotion State, the player has to release the crouch button AND be able to stand back up.
  (bind _stateactorcomponent (`/Game/RoadToTemehani/Core/StateManager/AC_PlayerStatesManager.GetStateActorComponent` _states_manager "NewEnumerator6"))
  (bind _ascrouch_locomotion_state (cast `/Game/RoadToTemehani/Player/States/AC_CrouchLocomotion_PS` _stateactorcomponent))
  (`/Game/RoadToTemehani/Core/StateManager/AC_PlayerStatesManager.SelectStateFromBool` _states_manager "NewEnumerator6" "NewEnumerator5" (or (not (`/Game/RoadToTemehani/Player/States/AC_CrouchLocomotion_PS.CanCharacterStandUp` _ascrouch_locomotion_state)) (`/Game/RoadToTemehani/Core/StateManager/AC_PlayerStatesManager.IsInputPressed` _states_manager "NewEnumerator2")))
  (return))

(fn `Update`
  (`parent.Update`)
  (return))