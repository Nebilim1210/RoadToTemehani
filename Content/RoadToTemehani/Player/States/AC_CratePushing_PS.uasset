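; Player state component for pushing crates, entered when a forward line trace finds a BP_PushableCrate.
; Enter slows the player, locks facing, nudges the crate ahead and attaches it; Exit reverts this.
; Movement input applies only when a box trace around the crate is clear, and the state ends on release or when either falls.
; A looping timer switches walk/idle flipbooks and the pushing loop sound based on movement.
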(fn `Enter`
  (params (PreviousState :type "/Game/RoadToTemehani/Core/StateManager/EPlayerStates Enum" :default "NewEnumerator7"))
  (bind _character_movement (`self.GetPlayerMovementComponent`))
  (bind _crateactor (`self.CrateActor`))
  (`parent.Enter` PreviousState)
  (add `/Game/RoadToTemehani/Player/BP_Player.OnPlayerStartFalling` (`self.Player Actor`) (`|CreateDelegate` :!event `OnPlayerStartFalling`)) ; Called to transition state when the player starts falling in the void
  ;[1 1 1] The player has to be slowed when he pushes the crate, and he must not turn around
  (set `CharacterMovementComponent.bOrientRotationToMovement` false _character_movement) ; While we're in that state, we want the player to keep facing the crate
  (bind _output_get (set `self.DefaultWalkSpeed` (`CharacterMovementComponent.MaxWalkSpeed` _character_movement))) ; Gets the current walk speed of the player
  (set `CharacterMovementComponent.MaxWalkSpeed` (* _output_get (`self.WalkSpeedScale`)) _character_movement) ; Changes the player's speed
  (`GameplayStatics.SpawnSound2D` (`self.PushingStartSFX`) 1.0 1.0 0.0 null)
  ;[1 1 1] Creates a timer that will update the animation every x frames
  (`self.UpdateCharacterAnimation`)
  (bind _returnvalue (`KismetSystemLibrary.K2_SetTimerDelegate` (`|CreateDelegate` :!event `UpdateCharacterAnimation`) (/ 1.0 (`self.AnimationRefreshRate`)) true)) ; Gives us X update of the animation if he's moving or not
  (set `self.AnimationTimerHandle` _returnvalue)
  (bind _sweephitresult (`Actor.K2_AddActorWorldOffset` _crateactor (`self.LocAdjustmentVector`) true false)) ; We move the crate sliiiightly before the player so he won't be stuck by it while pushing.\nNote : We could replace this node by a set collision response to channel.
  (bind (_bblockinghit _binitialoverlap _time _distance _location _impactpoint _normal _impactnormal _physmat _hitactor _hitcomponent _hitbonename _bonename _hititem _elementindex _faceindex _tracestart _traceend) (`GameplayStatics.BreakHitResult` _sweephitresult))
  ;[1 1 1] If the crate couldn't be moved because of an obstacle, we push the player back, away from the crate
  (if _bblockinghit
    (`Actor.K2_AddActorWorldOffset` (`self.Player Actor`) (- _location _traceend) true false))
  (`Actor.K2_AttachToActor` _crateactor (`self.Player Actor`) "None" "KeepWorld" "KeepWorld" "KeepWorld" true) ; Attach the crate to the player to follow it.
  (return))

(fn `Exit`
  (params (NextState :type "/Game/RoadToTemehani/Core/StateManager/EPlayerStates Enum" :default "NewEnumerator7"))
  (`parent.Exit` NextState)
  (remove `/Game/RoadToTemehani/Player/BP_Player.OnPlayerStartFalling` (`self.Player Actor`) (`|CreateDelegate` :!event `OnPlayerStartFalling`))
  (set `CharacterMovementComponent.bOrientRotationToMovement` true (`self.GetPlayerMovementComponent`)) ; When we exit the state, the player can turn around normally again
  (set `CharacterMovementComponent.MaxWalkSpeed` (`self.DefaultWalkSpeed`) (`self.GetPlayerMovementComponent`)) ; Changes the player's speed, so they go back to their normal speed
  (`KismetSystemLibrary.K2_ClearAndInvalidateTimerHandle` (`self.AnimationTimerHandle`))
  (`Actor.K2_DetachFromActor` (`self.CrateActor`) "KeepWorld" "KeepWorld" "KeepWorld")
  ;[1 1 1] Stops and deletes the crate loop sound playing before exiting the state
  (bind _pushingloopaudiocomp (`self.PushingLoopAudioComp`)
    (:`then`
      (`AudioComponent.Stop` _pushingloopaudiocomp)
      (`self.K2_DestroyComponent` _pushingloopaudiocomp))
    (:`else`
      _))
  (return))

(fn `FindCrate`
  (params (DistanceAlongX :type "Float (double-precision)"))
  (returns (OutHit :type "HitResult Structure") (FoundCrate :type Boolean))
  (bind _player_actor (`self.Player Actor`))
  (bind _returnvalue (`Actor.K2_GetActorLocation` _player_actor))
  (bind (_outhit _returnvalue_2) (`KismetSystemLibrary.LineTraceSingleForObjects` :`Start` _returnvalue :`End` (+ _returnvalue (* (`Actor.GetActorForwardVector` _player_actor) (+ DistanceAlongX (`CapsuleComponent.GetScaledCapsuleRadius` (`Character.CapsuleComponent` _player_actor))))) :`ObjectTypes` (`|MakeArray` "ObjectTypeQuery8" :!type "EObjectTypeQuery Enum") :`DrawDebugType` "ForDuration"))
  (bind (_bblockinghit _binitialoverlap _time _distance _location _impactpoint _normal _impactnormal _physmat _hitactor _hitcomponent _hitbonename _bonename _hititem _elementindex _faceindex _tracestart _traceend) (`GameplayStatics.BreakHitResult` _outhit))
  ;[1 1 1] If a crate has been found we keep a reference to it to attach it to the player during its movements.
  (bind _aspushable_crate (cast `/Game/RoadToTemehani/Placeables/Interactables/Crate/BP_PushableCrate` _hitactor)
    (:`then`
      (set `self.CrateActor` _aspushable_crate)
      (set `self.LocAdjustmentVector` (- _traceend _location)) ; Position difference to apply to the crate so it is positionned at the Distance CrateSearchDistance
      (return _outhit _returnvalue_2))
    (:`CastFailed`
      (return _outhit false))))

(fn `HandleInput`
  (params (InputType :type "/Game/RoadToTemehani/Core/StateManager/EPlayerInputs Enum" :default "NewEnumerator1") (bPressed :type Boolean))
  (returns (bChangeState :type Boolean) (TargetState :type "/Game/RoadToTemehani/Core/StateManager/EPlayerStates Enum"))
  (`parent.HandleInput` InputType bPressed)
  ;[1 1 1] Manages the movement while pushing the crate
  (bind (_inputtypepassthrough _bpressedpassthrough) (`/Game/RoadToTemehani/Core/StateManager/BPML_PlayerStatesUtilities.IsInputEqualTo?` InputType bPressed)
    (:`Yes`
      (`self.TryToMovePlayer` _bpressedpassthrough)
      ;[1 1 1] When the player moves, we check if the crate is in the void. If it is, we make it fall and leave the state
      (bind _bsuccess (`/Game/RoadToTemehani/Placeables/Interactables/Crate/BP_PushableCrate.TryToTriggerFalling` (`self.CrateActor`)))
      (if _bsuccess
        (return true "NewEnumerator5")
        (else
          (return false "NewEnumerator7"))))
    (:`No`
      ;[1 1 1] Ground locomotion after stopping pushing the crate
      (`/Game/RoadToTemehani/Core/StateManager/BPML_PlayerStatesUtilities.IsInputReleased?` _inputtypepassthrough _bpressedpassthrough "NewEnumerator6"
        (:`Yes`
          (return true "NewEnumerator5"))
        (:`No`
          (return false "NewEnumerator7"))))))

(fn `IsAccessible`
  (returns (bResult :type Boolean))
  (`parent.IsAccessible`)
  (bind (_outhit _foundcrate) (`self.FindCrate` (`self.CrateSearchDistance`)))
  (return _foundcrate))

(fn `OnPlayerStartFalling`
  (`/Game/RoadToTemehani/Core/StateManager/AC_PlayerStatesManager.HandleStateTransition` (`self.GetPlayerStatesManager`) "NewEnumerator9")
  (return))

(fn `TogglePushingLoopSFX`
  (params (bActivate :type Boolean))
  (if bActivate
    (bind _pushingloopaudiocomp (`self.PushingLoopAudioComp`)
      (:`then`
        ;[1 1 1] If the sound was already created we just play it back
        (if (not (`AudioComponent.IsPlaying` _pushingloopaudiocomp))
          (`AudioComponent.Play` _pushingloopaudiocomp 0.0)))
      (:`else`
        ;[1 1 1] Plays the sound and keeps a reference to him in order to pause him and play it whenever we want
        (bind _returnvalue (`GameplayStatics.SpawnSound2D` (`self.PushingLoopSFX`) 1.0 1.0 0.0 null false false))
        (set `self.PushingLoopAudioComp` _returnvalue)))
    (else
      ;[1 1 1] When the player is stopped, we stop the crate sound as well
      (bind _pushingloopaudiocomp_2 (`self.PushingLoopAudioComp`)
        (:`then`
          (if (`AudioComponent.IsPlaying` _pushingloopaudiocomp_2)
            (`AudioComponent.Stop` _pushingloopaudiocomp_2)))
        (:`else`
          _))))
  (return))

(fn `TryToMovePlayer`
  (params (bMoveRight :type Boolean))
  (bind _crateactor (`self.CrateActor`))
  (bind _returnvalue (`Actor.K2_GetActorLocation` _crateactor))
  (bind (_returnvalue_x _returnvalue_y _returnvalue_z) (`KismetMathLibrary.BreakVector` (`BoxComponent.GetScaledBoxExtent` (`/Game/RoadToTemehani/Placeables/Interactables/Crate/BP_PushableCrate.Box` _crateactor))))
  ;[1 1 1] Traces a box on the left or the right depending on the player's movements to check if the crates makes a collision with something or not.
  (bind (_outhit _returnvalue_2) (`KismetSystemLibrary.BoxTraceSingleByProfile` _returnvalue (`KismetMathLibrary.MakeVector` (+ (* (`KismetMathLibrary.SelectFloat` 1.0 -1.0 bMoveRight) (`self.BoxCollisionSearchDist`)) (.x _returnvalue)) (.y _returnvalue) (.z _returnvalue)) (`KismetMathLibrary.MakeVector` _returnvalue_x _returnvalue_y (- _returnvalue_z (`self.BoxCollisionSizeDifference`))) (struct) "Pawn" false (`|MakeArray` _crateactor (`self.Player Actor`) :!type "Actor Object Reference") "ForOneFrame"))
  ;[1 1 1] We move the player and the crate only if we found nothing
  (if (not _returnvalue_2)
    (`self.Add Movement Input` bMoveRight))
  (return))

(fn `UpdateCharacterAnimation`
  (bind _flipbook_manager (`self.GetPlayerFlipbookManager`))
  (if (or (> (`KismetMathLibrary.VSizeSquared` (`Actor.GetVelocity` (`self.Player Actor`))) 0.0) (> (`KismetMathLibrary.VSizeSquared` (`CharacterMovementComponent.GetCurrentAcceleration` (`self.GetPlayerMovementComponent`))) 0.0))
    (`/Game/RoadToTemehani/Core/FlipbookManager/AC_FlipbookManager.PlayLoopingAnimation` _flipbook_manager (`self.WalkFB`) "None")
    (`self.TogglePushingLoopSFX` true)
    (else
      (`/Game/RoadToTemehani/Core/FlipbookManager/AC_FlipbookManager.PlayLoopingAnimation` _flipbook_manager (`self.IdleFB`) "None")
      (`self.TogglePushingLoopSFX` false)))
  (return))