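; Player jump state component that launches the character, plays the jump flipbook and sound, and handles the airborne phase.
; Enter swaps walk speed to an air speed and Exit restores the cached ground speed.
; A looping timer, started on Enter and cleared on Exit, line-traces below the capsule and asks the states manager to transition once ground is near.
; Input only steers air movement and never changes state.
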(fn `ChangeSpeedStats`
  (params (Jumping :type Boolean))
  (set `CharacterMovementComponent.MaxWalkSpeed` (`KismetMathLibrary.SelectFloat` (`self.AirSpeed`) (`self.WalkSpeedStanding`) Jumping) (`self.GetPlayerMovementComponent`))
  (return))

(fn `Enter`
  (params (PreviousState :type "/Game/RoadToTemehani/Core/StateManager/EPlayerStates Enum" :default "NewEnumerator7"))
  (`parent.Enter` PreviousState)
  (set `self.WalkSpeedStanding` (`CharacterMovementComponent.MaxWalkSpeed` (`self.GetPlayerMovementComponent`))) ; Gets the current walk speed of the player
  (`self.ChangeSpeedStats` true)
  (`/Game/RoadToTemehani/Player/BP_Player.Launch` (`self.Player Actor`) (`self.JumpTrajectory`) (0.0 0.0 1.0) (0.0 0.0 0.0) false true)
  (`/Game/RoadToTemehani/Core/FlipbookManager/AC_FlipbookManager.PlayLoopingAnimation` (`self.GetPlayerFlipbookManager`) (`self.JumpFB`) "None")
  (`GameplayStatics.SpawnSound2D` (`self.JumpStartSfx`) 1.0 1.0 0.0 null)
  (`self.Start Trying to Land`)
  (return))

(fn `Exit`
  (params (NextState :type "/Game/RoadToTemehani/Core/StateManager/EPlayerStates Enum" :default "NewEnumerator7"))
  (`parent.Exit` NextState)
  (`self.StopTryingToLand`)
  (`self.ChangeSpeedStats` false)
  (return))

(fn `HandleInput`
  (params (InputType :type "/Game/RoadToTemehani/Core/StateManager/EPlayerInputs Enum" :default "NewEnumerator1") (bPressed :type Boolean))
  (returns (bChangeState :type Boolean) (TargetState :type "/Game/RoadToTemehani/Core/StateManager/EPlayerStates Enum"))
  (`parent.HandleInput` InputType bPressed)
  ;[1 1 1] Handles air horizontal movement
  (bind (_inputtypepassthrough _bpressedpassthrough) (`/Game/RoadToTemehani/Core/StateManager/BPML_PlayerStatesUtilities.IsInputEqualTo?` InputType bPressed)
    (:`Yes`
      (`self.Add Movement Input` _bpressedpassthrough)
      (return false "NewEnumerator7"))
    (:`No`
      (return false "NewEnumerator7"))))

(fn `IsCharacterLanded`
  (returns (ReturnValue :type Boolean))
  (bind _returnvalue (`Actor.K2_GetActorLocation` (`self.Player Actor`)))
  (bind (_outhit _returnvalue_2) (`KismetSystemLibrary.LineTraceSingleByProfile` _returnvalue (- _returnvalue (`KismetMathLibrary.MakeVector` 0.0 0.0 (+ (`CapsuleComponent.CapsuleHalfHeight` (`Character.CapsuleComponent` (`self.Player Actor`))) (`self.DistanceToGroundForLanding`)))) "Pawn"))
  (return _returnvalue_2))

(fn `Start Trying to Land`
  (bind _returnvalue (`KismetSystemLibrary.K2_SetTimerDelegate` (`|CreateDelegate` :!event `TryToLand`) (/ 1.0 (`self.NBLandingTriesPerSecond`)) true))
  (set `self.LandingTimerHandle` _returnvalue)
  (return))

(fn `StopTryingToLand`
  (`KismetSystemLibrary.K2_ClearAndInvalidateTimerHandle` (`self.LandingTimerHandle`))
  (return))

(fn `TryToLand`
  (if (`self.IsCharacterLanded`)
    (`/Game/RoadToTemehani/Core/StateManager/AC_PlayerStatesManager.HandleStateTransition` (`self.GetPlayerStatesManager`) "NewEnumerator5"))
  (return))