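; Player state component for gliding in a state-machine-driven character controller.
; On enter it applies glide gravity, zeroes vertical velocity and plays a looping flipbook and sound, then routes input to air movement or transitions like double jump, drop and dive.
; Landing picks a ground state, and moving toward a found wall triggers a wall grab.
; Exiting starts a cooldown that re-enables gliding, retrying if the input is held; landing also re-enables it.
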(event `self.ReceiveBeginPlay`
  ;[1 1 1] Begin play : each time the player will touch the ground, we reactivate the possibility of double jumping, no matter the state we will be in when we land.
  (`parent.ReceiveBeginPlay`)
  (add `/Game/RoadToTemehani/Player/BP_Player.OnPlayerLanded` (`self.Player Actor`) (delegate `EnableGlideEvent`)))

(event `EnableGlideEvent`
  (params (Hit :type "HitResult Structure"))
  ;[1 1 1] Begin play : each time the player will touch the ground, we reactivate the possibility of double jumping, no matter the state we will be in when we land.
  (set `self.bCanGlide` true))

(fn `EnableGlide`
  (bind _states_manager (`self.GetPlayerStatesManager`))
  ;[1 1 1] Once the glide cooldown is over, enables the player to glide, and tries to glide immediately if the gliding key is pressed.
  (set `self.bCanGlide` true)
  (if (`/Game/RoadToTemehani/Core/StateManager/AC_PlayerStatesManager.IsInputPressed` _states_manager "NewEnumerator4")
    (`/Game/RoadToTemehani/Core/StateManager/AC_PlayerStatesManager.HandlePlayerInput` _states_manager "NewEnumerator4" true))
  (return))

(fn `Enter`
  (params (PreviousState :type "/Game/RoadToTemehani/Core/StateManager/EPlayerStates Enum" :default "NewEnumerator7"))
  (`parent.Enter` PreviousState)
  (add `/Game/RoadToTemehani/Player/BP_Player.OnPlayerLanded` (`self.Player Actor`) (`|CreateDelegate` :!event `On Player Landed`))
  (`/Game/RoadToTemehani/Player/BP_Player.UpdateGravityScale` (`self.Player Actor`) (`self.TrajectoryParameters`))
  (`self.StopPlayerVelocityZ`)
  (`/Game/RoadToTemehani/Core/FlipbookManager/AC_FlipbookManager.PlayLoopingAnimation` (`self.GetPlayerFlipbookManager`) (`self.Glide_FB`) "None")
  (`GameplayStatics.SpawnSound2D` (`self.GlideStartSfx`) 1.0 1.0 0.0 null)
  (return))

(fn `Exit`
  (params (NextState :type "/Game/RoadToTemehani/Core/StateManager/EPlayerStates Enum" :default "NewEnumerator7"))
  (`parent.Exit` NextState)
  (remove `/Game/RoadToTemehani/Player/BP_Player.OnPlayerLanded` (`self.Player Actor`) (`|CreateDelegate` :!event `On Player Landed`))
  (set `self.bCanGlide` false)
  (`KismetSystemLibrary.K2_SetTimerDelegate` (`|CreateDelegate` :!event `EnableGlide`) (`self.CooldownBetweenGlides`))
  (return))

(fn `HandleInput`
  (params (InputType :type "/Game/RoadToTemehani/Core/StateManager/EPlayerInputs Enum" :default "NewEnumerator1") (bPressed :type Boolean))
  (returns (bChangeState :type Boolean) (TargetState :type "/Game/RoadToTemehani/Core/StateManager/EPlayerStates Enum"))
  (`parent.HandleInput` InputType bPressed)
  ;[1 1 1] Handles Air horizontal movement
  (bind (_inputtypepassthrough _bpressedpassthrough) (`/Game/RoadToTemehani/Core/StateManager/BPML_PlayerStatesUtilities.IsInputEqualTo?` InputType bPressed)
    (:`Yes`
      (`self.Add Movement Input` _bpressedpassthrough)
      (return false "NewEnumerator7"))
    (:`No`
      ;[1 1 1] Handles Double Jump
      (bind (_inputtypepassthrough_2 _bpressedpassthrough_2) (`/Game/RoadToTemehani/Core/StateManager/BPML_PlayerStatesUtilities.IsInputPressed?` _inputtypepassthrough _bpressedpassthrough "NewEnumerator3")
        (:`Yes`
          (return true "NewEnumerator10"))
        (:`No`
          ;[1 1 1] Handles Gliding Drop
          (bind (_inputtypepassthrough_3 _bpressedpassthrough_3) (`/Game/RoadToTemehani/Core/StateManager/BPML_PlayerStatesUtilities.IsInputReleased?` _inputtypepassthrough_2 _bpressedpassthrough_2 "NewEnumerator4")
            (:`Yes`
              (return true "NewEnumerator9"))
            (:`No`
              ;[1 1 1] Handles Diving transition
              (`/Game/RoadToTemehani/Core/StateManager/BPML_PlayerStatesUtilities.IsInputPressed?` _inputtypepassthrough_3 _bpressedpassthrough_3 "NewEnumerator6"
                (:`Yes`
                  (return true "NewEnumerator17"))
                (:`No`
                  (return false "NewEnumerator7"))))))))))

(fn `IsAccessible`
  (returns (bResult :type Boolean))
  (`parent.IsAccessible`)
  (return (`self.bCanGlide`)))

(fn `On Player Landed`
  (params (Hit :type "HitResult Structure"))
  (`/Game/RoadToTemehani/Core/StateManager/AC_PlayerStatesManager.SelectStateFromInputPressed` (`self.GetPlayerStatesManager`) "NewEnumerator6" "NewEnumerator5" "NewEnumerator2")
  (`self.EnableGlide`)
  (return))

(fn `OnWallFound`
  ;[1 1 1] If the player is close to a wall and he moves towards this wall (tilting the stick), as he also presses the glide, he'll wall grab.
  (`parent.OnWallFound`)
  (if (`self.IsPlayerMovingTowardsWall`)
    (`/Game/RoadToTemehani/Core/StateManager/AC_PlayerStatesManager.HandleStateTransition` (`self.GetPlayerStatesManager`) "NewEnumerator14"))
  (return))

(fn `StopPlayerVelocityZ`
  (bind _character_movement (`self.GetPlayerMovementComponent`))
  (bind (_velocity_x _velocity_y) (`KismetMathLibrary.BreakVector` (`MovementComponent.Velocity` _character_movement)))
  (set `MovementComponent.Velocity` (`KismetMathLibrary.MakeVector` _velocity_x _velocity_y) _character_movement)
  (return))