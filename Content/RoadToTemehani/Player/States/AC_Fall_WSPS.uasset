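; Player state component for falling, which sets fall gravity from trajectory parameters and plays a looping fall flipbook on entry.
; Input handling applies air movement or switches state to wall jump when near a wall, double jump otherwise, or glide.
; It binds to the player's landed event while active; landing spawns run or idle dust by X velocity and picks the next state from held input.
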(fn `Enter`
  (params (PreviousState :type "/Game/RoadToTemehani/Core/StateManager/EPlayerStates Enum" :default "NewEnumerator7"))
  (`parent.Enter` PreviousState)
  (add `/Game/RoadToTemehani/Player/BP_Player.OnPlayerLanded` (`self.Player Actor`) (`|CreateDelegate` :!event `OnPlayerLanded`))
  (`/Game/RoadToTemehani/Player/BP_Player.UpdateGravityScale` (`self.Player Actor`) (`self.TrajectoryParameters`))
  (`/Game/RoadToTemehani/Core/FlipbookManager/AC_FlipbookManager.PlayLoopingAnimation` (`/Game/RoadToTemehani/Player/BP_Player.Flipbook Manager` (`self.Player Actor`)) (`self.FallFB`) "None")
  (return))

(fn `Exit`
  (params (NextState :type "/Game/RoadToTemehani/Core/StateManager/EPlayerStates Enum" :default "NewEnumerator7"))
  (`parent.Exit` NextState)
  (remove `/Game/RoadToTemehani/Player/BP_Player.OnPlayerLanded` (`self.Player Actor`) (`|CreateDelegate` :!event `OnPlayerLanded`))
  (return))

(fn `GenerateLandDust`
  (bind _player_actor (`self.Player Actor`))
  (bind _returnvalue_x (`KismetMathLibrary.BreakVector` (`Actor.GetVelocity` _player_actor)))
  (`NiagaraFunctionLibrary.SpawnSystemAttached` (select `bool` (!= _returnvalue_x 0.0) :`false` (`self.LandDustIdleVFX`) :`true` (`self.LandDustRunVFX`)) (`Character.CapsuleComponent` _player_actor) "None" (0.0 0.0 0.0) (struct) "KeepRelativeOffset" true)
  (return))

(fn `HandleInput`
  (params (InputType :type "/Game/RoadToTemehani/Core/StateManager/EPlayerInputs Enum" :default "NewEnumerator1") (bPressed :type Boolean))
  (returns (bChangeState :type Boolean) (TargetState :type "/Game/RoadToTemehani/Core/StateManager/EPlayerStates Enum"))
  (`parent.HandleInput` InputType bPressed)
  ;[1 1 1] Handles Air horizontal movement
  (bind (_inputtypepassthrough _bpressedpassthrough) (`/Game/RoadToTemehani/Core/StateManager/BPML_PlayerStatesUtilities.IsInputEqualTo?` InputType bPressed)
    (:`Yes`
      (`self.Add Movement Input` _bpressedpassthrough)
      (return false "NewEnumerator7"))
    (:`No`
      ;[1 1 1] Handles Double Jump and Wall Jump
      (bind (_inputtypepassthrough_2 _bpressedpassthrough_2) (`/Game/RoadToTemehani/Core/StateManager/BPML_PlayerStatesUtilities.IsInputPressed?` _inputtypepassthrough _bpressedpassthrough "NewEnumerator3")
        (:`Yes`
          (if (`self.IsPlayerCloseToA_Wall`)
            ;[1 1 1] Handles Wall Jump
            (return true "NewEnumerator12")
            (else
              (return true "NewEnumerator10"))))
        (:`No`
          ;[1 1 1] Handles Gliding Transition
          (`/Game/RoadToTemehani/Core/StateManager/BPML_PlayerStatesUtilities.IsInputPressed?` _inputtypepassthrough_2 _bpressedpassthrough_2 "NewEnumerator4"
            (:`Yes`
              (return true "NewEnumerator11"))
            (:`No`
              (return false "NewEnumerator7"))))))))

(fn `OnPlayerLanded`
  (params (Hit :type "HitResult Structure"))
  (`self.GenerateLandDust`)
  (`/Game/RoadToTemehani/Core/StateManager/AC_PlayerStatesManager.SelectStateFromInputPressed` (`self.GetPlayerStatesManager`) "NewEnumerator6" "NewEnumerator5" "NewEnumerator2")
  (return))