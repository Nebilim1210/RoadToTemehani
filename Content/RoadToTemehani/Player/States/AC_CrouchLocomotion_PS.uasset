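; Player state for crouched idle and walking, with flipbook animation, footstep sounds and exits to standing, jump, ground slide or falling.
; Enter and Exit toggle walk speed, capsule height and sprite offset, skipping the resize when coming from or going to a ground slide.
; A looping timer picks the idle or walk flipbook.
; Releasing crouch under an obstacle starts a timer that repeats an upward line trace until standing is possible.
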(fn `CanCharacterStandUp`
  (returns (bResult :type Boolean))
  (bind _returnvalue (`Actor.K2_GetActorLocation` (`self.Player Actor`)))
  (bind (_outhit _returnvalue_2) (`KismetSystemLibrary.LineTraceSingleByProfile` _returnvalue (+ _returnvalue (`KismetMathLibrary.MakeVector` 0.0 0.0 (+ (- (* (`self.CapsuleHalfHeightStanding`) 2.0) (`self.CapsuleHalfHeightCrouched`)) (`self.StandUpTraceLength`)))) "Pawn"))
  (return (not _returnvalue_2)))

(fn `Enter`
  (params (PreviousState :type "/Game/RoadToTemehani/Core/StateManager/EPlayerStates Enum" :default "NewEnumerator7"))
  (bind (_relativelocation_x _relativelocation_y _relativelocation_z) (`KismetMathLibrary.BreakVector` (`SceneComponent.RelativeLocation` (`self.GetPlayerFlipbookComponent`))))
  (`parent.Enter` PreviousState)
  (add `/Game/RoadToTemehani/Core/FlipbookManager/AC_FlipbookManager.OnTrackedFrameFound` (`self.GetPlayerFlipbookManager`) (`|CreateDelegate` :!event `OnFootstepFramedReached`))
  (add `/Game/RoadToTemehani/Player/BP_Player.OnPlayerStartFalling` (`self.Player Actor`) (`|CreateDelegate` :!event `OnPlayerStartFalling`))
  (`GameplayStatics.SpawnSound2D` (`self.CrouchStartSFX`) 1.0 1.0 0.0 null)
  ;[1 1 1] If we come from the ground slide, as we are already in a crouched mode, we don't need to crouch again. Else we crouch and lower our speed.
  (if (`|EnumInequality` PreviousState "NewEnumerator16")
    (set `self.WalkSpeedStanding` (`CharacterMovementComponent.MaxWalkSpeed` (`self.GetPlayerMovementComponent`))) ; Gets the current walk speed of the player
    (set `self.SpriteRelLocationStanding` _relativelocation_z) ; Gets the sprite's position for the upstanding player
    (set `self.CapsuleHalfHeightStanding` (`CapsuleComponent.CapsuleHalfHeight` (`Character.CapsuleComponent` (`self.Player Actor`)))) ; Gets the default capsule half height to use when the player gets up
    (`self.Toggle Crouch` true)
    (elif (not (`/Game/RoadToTemehani/Core/StateManager/AC_PlayerStatesManager.IsInputPressed` (`self.GetPlayerStatesManager`) "NewEnumerator2"))
      (`self.StartTryingToStandUp`)))
  ;[1 1 1] Creates a timer that will update the animation every x frames
  (`self.UpdateCharacterAnimation`)
  (bind _returnvalue (`KismetSystemLibrary.K2_SetTimerDelegate` (`|CreateDelegate` :!event `UpdateCharacterAnimation`) (/ 1.0 (`self.AnimUpdatesPerSecond`)) true))
  (set `self.AnimationTimerHandle` _returnvalue)
  (return))

(fn `Exit`
  (params (NextState :type "/Game/RoadToTemehani/Core/StateManager/EPlayerStates Enum" :default "NewEnumerator7"))
  (`parent.Exit` NextState)
  (remove `/Game/RoadToTemehani/Core/FlipbookManager/AC_FlipbookManager.OnTrackedFrameFound` (`self.GetPlayerFlipbookManager`) (`|CreateDelegate` :!event `OnFootstepFramedReached`))
  (remove `/Game/RoadToTemehani/Player/BP_Player.OnPlayerStartFalling` (`self.Player Actor`) (`|CreateDelegate` :!event `OnPlayerStartFalling`))
  (`self.StopTryingToStandUp`)
  (`KismetSystemLibrary.K2_ClearAndInvalidateTimerHandle` (`self.AnimationTimerHandle`))
  ;[1 1 1] If we transition towards ground slide, then we don't resize the capsule
  (if (`|EnumInequality` NextState "NewEnumerator16")
    (`self.Toggle Crouch` false))
  (return))

(fn `HandleInput`
  (params (InputType :type "/Game/RoadToTemehani/Core/StateManager/EPlayerInputs Enum" :default "NewEnumerator1") (bPressed :type Boolean))
  (returns (bChangeState :type Boolean) (TargetState :type "/Game/RoadToTemehani/Core/StateManager/EPlayerStates Enum"))
  (`parent.HandleInput` InputType bPressed)
  ;[1 1 1] Handles transitioning back to uncrouched standing state if crouch key is released
  (bind (_inputtypepassthrough _inputpressedpassthrough) (`/Game/RoadToTemehani/Core/StateManager/BPML_PlayerStatesUtilities.CompareInputEventTo` InputType bPressed "NewEnumerator2")
    (:`Pressed`
      (`self.StopTryingToStandUp`)
      (return false "NewEnumerator5"))
    (:`Released`
      (if (`self.CanCharacterStandUp`)
        (return true "NewEnumerator5")
        (else
          (`self.StartTryingToStandUp`)
          (return false "NewEnumerator5"))))
    (:`Unused`
      ;[1 1 1] Manages movement while crouched
      (bind (_inputtypepassthrough_2 _bpressedpassthrough) (`/Game/RoadToTemehani/Core/StateManager/BPML_PlayerStatesUtilities.IsInputEqualTo?` _inputtypepassthrough _inputpressedpassthrough)
        (:`Yes`
          (`self.Add Movement Input` _bpressedpassthrough)
          (return false "NewEnumerator5"))
        (:`No`
          ;[1 1 1] Manages jumping from crouched state
          (bind (_inputtypepassthrough_3 _bpressedpassthrough_2) (`/Game/RoadToTemehani/Core/StateManager/BPML_PlayerStatesUtilities.IsInputPressed?` _inputtypepassthrough_2 _bpressedpassthrough "NewEnumerator3")
            (:`Yes`
              (return true "NewEnumerator8"))
            (:`No`
              ;[1 1 1] Manages Ground sliding from crouched state
              (`/Game/RoadToTemehani/Core/StateManager/BPML_PlayerStatesUtilities.IsInputPressed?` _inputtypepassthrough_3 _bpressedpassthrough_2 "NewEnumerator5"
                (:`Yes`
                  (return true "NewEnumerator16"))
                (:`No`
                  (return false "NewEnumerator7"))))))))))

(fn `OnFootstepFramedReached`
  (params (FrameIndex :type Integer))
  (`GameplayStatics.SpawnSound2D` (`self.CrouchWalkSFX`) 1.0 1.0 0.0 null)
  (return))

(fn `OnPlayerStartFalling`
  (`/Game/RoadToTemehani/Core/StateManager/AC_PlayerStatesManager.HandleStateTransition` (`self.GetPlayerStatesManager`) "NewEnumerator9")
  (return))

(fn `StartTryingToStandUp`
  (`self.TryToStandUp`)
  (bind _returnvalue (`KismetSystemLibrary.K2_SetTimerDelegate` (`|CreateDelegate` :!event `TryToStandUp`) (/ 1.0 (`self.NbStandUpTriesPerSecond`)) true))
  (set `self.StandUpTimerHandle` _returnvalue)
  (return))

(fn `StopTryingToStandUp`
  (`KismetSystemLibrary.K2_ClearAndInvalidateTimerHandle` (`self.StandUpTimerHandle`))
  (return))

(fn `Toggle Crouch`
  (params (`bShould Crouch` :type Boolean))
  (locals (L_ShouldCrouch :type Boolean))
  (bind _returnvalue (- (`self.CapsuleHalfHeightStanding`) (`self.CapsuleHalfHeightCrouched`)))
  ;[1 1 1] Changes the movement speed of the player
  (set `local.L_ShouldCrouch` `bShould Crouch`)
  (set `CharacterMovementComponent.MaxWalkSpeed` (`KismetMathLibrary.SelectFloat` (`self.WalkSpeedCrouched`) (`self.WalkSpeedStanding`) (`local.L_ShouldCrouch`)) (`self.GetPlayerMovementComponent`))
  ;[1 1 1] Changes the player's sprite position accordingly to avoid him melting in the ground
  (`SceneComponent.K2_SetRelativeLocation` (`self.GetPlayerFlipbookComponent`) (`KismetMathLibrary.MakeVector` 0.0 0.0 (`KismetMathLibrary.SelectFloat` (`self.SpriteRelLocationCrouched`) (`self.SpriteRelLocationStanding`) (`local.L_ShouldCrouch`))) false true)
  ;[1 1 1] Changes the Capsule half height in a crouch
  (`CapsuleComponent.SetCapsuleHalfHeight` (`Character.CapsuleComponent` (`self.Player Actor`)) (`KismetMathLibrary.SelectFloat` (`self.CapsuleHalfHeightCrouched`) (`self.CapsuleHalfHeightStanding`) (`local.L_ShouldCrouch`)) false)
  ;[1 1 1] Makes sure the capsule stays grounded
  (`SceneComponent.K2_AddWorldOffset` (`Character.CapsuleComponent` (`self.Player Actor`)) (`KismetMathLibrary.MakeVector` 0.0 0.0 (`KismetMathLibrary.SelectFloat` (* _returnvalue -1.0) _returnvalue (`local.L_ShouldCrouch`))) false true)
  (return))

(fn `TryToStandUp`
  (if (`self.CanCharacterStandUp`)
    (`/Game/RoadToTemehani/Core/StateManager/AC_PlayerStatesManager.HandleStateTransition` (`self.GetPlayerStatesManager`) "NewEnumerator5"))
  (return))

(fn `UpdateCharacterAnimation`
  (bind _flipbook_manager (`self.GetPlayerFlipbookManager`))
  (if (or (> (`KismetMathLibrary.VSizeXYSquared` (`Actor.GetVelocity` (`self.Player Actor`))) 0.0) (> (`KismetMathLibrary.VSizeSquared` (`CharacterMovementComponent.GetCurrentAcceleration` (`self.GetPlayerMovementComponent`))) 0.0))
    (`/Game/RoadToTemehani/Core/FlipbookManager/AC_FlipbookManager.PlayLoopingAnimationAndTrackFrames` _flipbook_manager (`self.CrouchWalkFB`) "None" (`|MakeArray` 5))
    (else
      (`/Game/RoadToTemehani/Core/FlipbookManager/AC_FlipbookManager.PlayLoopingAnimation` _flipbook_manager (`self.CrouchIdleFB`) "None")))
  (return))