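; Player state for the dive move, which drives the player straight down with a smooth movement, looping dive flipbook and start sound.
; A blocking hit during movement, or floor found when it finishes, triggers landing: walking mode, montage, sound, VFX, camera shake and a landed broadcast.
; The state manager picks the next state from input when the landing animation ends or the dive finishes without floor.
; Older trace-distance and recovery-timer logic remains disconnected.
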(fn `AfterLandingRecovery`
  (`KismetSystemLibrary.PrintString` "recovery over")
  (`/Game/RoadToTemehani/Core/StateManager/AC_PlayerStatesManager.SelectStateFromInputPressed` (`self.GetPlayerStatesManager`) "NewEnumerator6" "NewEnumerator5" "NewEnumerator2")
  (return))

(fn `Enter`
  (params (PreviousState :type "/Game/RoadToTemehani/Core/StateManager/EPlayerStates Enum" :default "NewEnumerator7"))
  (`parent.Enter` PreviousState)
  (add `/Game/RoadToTemehani/Player/BP_Player.OnSmoothMovementFinished` (`self.Player Actor`) (`|CreateDelegate` :!event `OnSmoothMovementFinished`)) ; Called when the player reaches the end of hiss movement, but did not touch anything.
  (add `/Game/RoadToTemehani/Player/BP_Player.OnSmoothMovementTick` (`self.Player Actor`) (`|CreateDelegate` :!event `OnSmoothMovementTick`)) ; Called on each frame of the smooth movement
  (add `/Game/RoadToTemehani/Core/FlipbookManager/AC_FlipbookManager.OnAnimationPlaybackFinished` (`self.GetPlayerFlipbookManager`) (`|CreateDelegate` :!event `OnAnimationPlaybackFinished`)) ; Called when the landing animation is done playing
  (`/Game/RoadToTemehani/Player/BP_Player.TriggerSmoothMovement` (`self.Player Actor`) (`KismetMathLibrary.MakeVector` 0.0 0.0 (* (`self.MaxDistance`) -1.0)) (`self.Duration`) "NewEnumerator1") ; Throws the player downards at max speed
  (`/Game/RoadToTemehani/Core/FlipbookManager/AC_FlipbookManager.PlayLoopingAnimation` (`self.GetPlayerFlipbookManager`) (`self.DiveLoopFB`) "None")
  (`GameplayStatics.SpawnSound2D` (`self.DiveStartSFX`) 1.0 1.0 0.0 null)
  (return))

(fn `Exit`
  (params (NextState :type "/Game/RoadToTemehani/Core/StateManager/EPlayerStates Enum" :default "NewEnumerator7"))
  (`parent.Exit` NextState)
  (remove `/Game/RoadToTemehani/Player/BP_Player.OnSmoothMovementFinished` (`self.Player Actor`) (`|CreateDelegate` :!event `OnSmoothMovementFinished`))
  (remove `/Game/RoadToTemehani/Player/BP_Player.OnSmoothMovementTick` (`self.Player Actor`) (`|CreateDelegate` :!event `OnSmoothMovementTick`))
  (remove `/Game/RoadToTemehani/Core/FlipbookManager/AC_FlipbookManager.OnAnimationPlaybackFinished` (`self.GetPlayerFlipbookManager`) (`|CreateDelegate` :!event `OnAnimationPlaybackFinished`))
  (return))

(fn `FindDiveDistance`
  (returns (FloatDistance :type Integer) (ReturnValue :type Boolean))
  (bind _player_actor (`self.Player Actor`))
  (bind _returnvalue (- (`Actor.K2_GetActorLocation` _player_actor) (`KismetMathLibrary.MakeVector` 0.0 0.0 (`CapsuleComponent.CapsuleHalfHeight` (`Character.CapsuleComponent` _player_actor)))))
  (bind (_outhit _returnvalue_2) (`KismetSystemLibrary.LineTraceSingleByProfile` :`Start` _returnvalue :`End` (- _returnvalue (`KismetMathLibrary.MakeVector` 0.0 0.0 (`self.DiveSearchDistance`))) :`ProfileName` "Pawn" :`DrawDebugType` "ForDuration"))
  (return (`KismetMathLibrary.FCeil` (`.Distance` (`GameplayStatics.BreakHitResult` _outhit))) _returnvalue_2))

(fn `OnAnimationPlaybackFinished`
  (params (Tag :type Name))
  (if (== Tag "Landed")
    (`/Game/RoadToTemehani/Core/StateManager/AC_PlayerStatesManager.SelectStateFromInputPressed` (`self.GetPlayerStatesManager`) "NewEnumerator6" "NewEnumerator5" "NewEnumerator2"))
  (return))

(fn `OnPlayerLanded`
  (`CharacterMovementComponent.SetMovementMode` (`self.GetPlayerMovementComponent`) "MOVE_Walking" 0) ; Avoid player's bounces if we dive too low
  (`/Game/RoadToTemehani/Core/FlipbookManager/AC_FlipbookManager.PlayMontage` (`self.GetPlayerFlipbookManager`) (`self.DiveLandFB`) "Landed")
  (`GameplayStatics.SpawnSound2D` (`self.DiveLandSFX`) 1.0 1.0 0.0 null)
  (`/Game/RoadToTemehani/Player/BP_Player.OnPlayerLanded` :`self` (`self.Player Actor`)) ; Warns all other states that the player has landed
  (`GameplayStatics.PlayWorldCameraShake` (`self.CameraShake`) (`Actor.K2_GetActorLocation` (`self.Player Actor`)) 20000.0 30000.0) ; Shakes the camera to give the impression of a powerful impact
  (`NiagaraFunctionLibrary.SpawnSystemAttached` (`self.DiveLandVFX`) (`Character.CapsuleComponent` (`self.Player Actor`)) "None" (0.0 0.0 0.0) (struct) "KeepRelativeOffset" true)
  (return))

(fn `OnSmoothMovementFinished`
  (bind _player_actor (`self.Player Actor`))
  (bind _floorresult_bblockinghit (break `FindFloorResult` (`CharacterMovementComponent.K2_FindFloor` (`Character.CharacterMovement` _player_actor) (`Actor.K2_GetActorLocation` _player_actor))))
  (if _floorresult_bblockinghit
    (`self.OnPlayerLanded`)
    (else
      (`/Game/RoadToTemehani/Core/StateManager/AC_PlayerStatesManager.SelectStateFromInputPressed` (`self.GetPlayerStatesManager`) "NewEnumerator11" "NewEnumerator9" "NewEnumerator4")))
  (return))

(fn `OnSmoothMovementTick`
  (params (HitResult :type "HitResult Structure"))
  (if (`GameplayStatics.BreakHitResult` HitResult)
    (`/Game/RoadToTemehani/Player/BP_Player.StopSmoothMovement` (`self.Player Actor`))
    (`self.OnPlayerLanded`))
  (return))

(fn `ShakeCamera`
  (`KismetSystemLibrary.PrintString` "Let's Shake the camera !")
  (`PlayerController.ClientStartCameraShake` :`self` (`GameplayStatics.GetPlayerController` 0) :`Shake` (`self.CameraShake`))
  (return))