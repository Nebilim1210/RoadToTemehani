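; Player state component for the double jump: on entry it launches the player along a configured trajectory with start flipbook, sound and Niagara effect, then loops the rising animation.
; It is accessible once per airtime, re-enabled by a landing listener bound at BeginPlay whatever the current state.
; While active it allows air movement and glide input, and transitions on reaching the jump apex or landing, binding those events only between Enter and Exit.
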(event `self.ReceiveBeginPlay`
  ;[1 1 1] Begin play : each time the player will touch the ground, we reactivate the possibility of double jumping, no matter the state we will be in when we land.
  (`parent.ReceiveBeginPlay`)
  (add `/Game/RoadToTemehani/Player/BP_Player.OnPlayerLanded` (`self.Player Actor`) (delegate `EnableDoubleJump`)))

(event `EnableDoubleJump`
  (params (Hit :type "HitResult Structure"))
  ;[1 1 1] Begin play : each time the player will touch the ground, we reactivate the possibility of double jumping, no matter the state we will be in when we land.
  (set `self.bCanDoubleJump` true))

(fn `Enter`
  (params (PreviousState :type "/Game/RoadToTemehani/Core/StateManager/EPlayerStates Enum" :default "NewEnumerator7"))
  (`parent.Enter` PreviousState)
  (add `/Game/RoadToTemehani/Core/FlipbookManager/AC_FlipbookManager.OnAnimationPlaybackFinished` (`self.GetPlayerFlipbookManager`) (`|CreateDelegate` :!event `OnAnimMontageFinished`))
  (add `/Game/RoadToTemehani/Player/BP_Player.OnPlayerLanded` (`self.Player Actor`) (`|CreateDelegate` :!event `OnPlayerLanded`))
  (add `Character.OnReachedJumpApex` (`self.Player Actor`) (`|CreateDelegate` :!event `OnPlayerReachedApex`))
  (set `CharacterMovementComponent.bNotifyApex` true (`self.GetPlayerMovementComponent`))
  (set `self.bCanDoubleJump` false) ; We can't double jump while we haven't touched the ground
  (`/Game/RoadToTemehani/Player/BP_Player.Launch` (`self.Player Actor`) (`self.TrajectoryParameters`) (0.0 0.0 1.0) (0.0 0.0 0.0) false true) ; Ejects the player in the airs
  (`/Game/RoadToTemehani/Core/FlipbookManager/AC_FlipbookManager.PlayMontage` (`self.GetPlayerFlipbookManager`) (`self.DoubleJumpStartFB`) "DoubleJumpStart")
  (`GameplayStatics.SpawnSound2D` (`self.DoubleJumpStartSFX`) 1.0 1.0 0.0 null)
  (`NiagaraFunctionLibrary.SpawnSystemAtLocation` (`self.DoubleJumpVfx`) (`Actor.K2_GetActorLocation` (`self.Player Actor`)))
  (return))

(fn `Exit`
  (params (NextState :type "/Game/RoadToTemehani/Core/StateManager/EPlayerStates Enum" :default "NewEnumerator7"))
  (bind _player_actor (`self.Player Actor`))
  (`parent.Exit` NextState)
  (remove `/Game/RoadToTemehani/Core/FlipbookManager/AC_FlipbookManager.OnAnimationPlaybackFinished` (`self.GetPlayerFlipbookManager`) (`|CreateDelegate` :!event `OnAnimMontageFinished`))
  (remove `/Game/RoadToTemehani/Player/BP_Player.OnPlayerLanded` _player_actor (`|CreateDelegate` :!event `OnPlayerLanded`))
  (remove `Character.OnReachedJumpApex` _player_actor (`|CreateDelegate` :!event `OnPlayerReachedApex`))
  (set `CharacterMovementComponent.bNotifyApex` false (`self.GetPlayerMovementComponent`))
  (return))

(fn `HandleInput`
  (params (InputType :type "/Game/RoadToTemehani/Core/StateManager/EPlayerInputs Enum" :default "NewEnumerator1") (bPressed :type Boolean))
  (returns (bChangeState :type Boolean) (TargetState :type "/Game/RoadToTemehani/Core/StateManager/EPlayerStates Enum"))
  (`parent.HandleInput` InputType bPressed)
  ;[1 1 1] Handles Air horizontal movement
  (bind (_inputtypepassthrough _bpressedpassthrough) (`/Game/RoadToTemehani/Core/StateManager/BPML_PlayerStatesUtilities.IsInputEqualTo?` InputType bPressed)
    (:`Yes`
      (`self.Add Movement Input` _bpressedpassthrough)
      (return false "NewEnumerator7"))
    (:`No`
      ;[1 1 1] Handles Glide Transition
      (`/Game/RoadToTemehani/Core/StateManager/BPML_PlayerStatesUtilities.IsInputPressed?` _inputtypepassthrough _bpressedpassthrough "NewEnumerator4"
        (:`Yes`
          (return true "NewEnumerator11"))
        (:`No`
          (return false "NewEnumerator7"))))))

(fn `IsAccessible`
  (returns (bResult :type Boolean))
  ;[1 1 1] We can only double jump once per fall
  (`parent.IsAccessible`)
  (return (`self.bCanDoubleJump`)))

(fn `OnAnimMontageFinished`
  (params (Tag :type Name))
  ;[1 1 1] Plays the double jump's animation's second face
  (if (== Tag "DoubleJumpStart")
    (`/Game/RoadToTemehani/Core/FlipbookManager/AC_FlipbookManager.PlayLoopingAnimation` (`self.GetPlayerFlipbookManager`) (`self.DoubleJumpUpLoopFB`) "None"))
  (return))

(fn `OnPlayerLanded`
  (params (Hit :type "HitResult Structure"))
  (`/Game/RoadToTemehani/Core/StateManager/AC_PlayerStatesManager.SelectStateFromInputPressed` (`self.GetPlayerStatesManager`) "NewEnumerator6" "NewEnumerator5" "NewEnumerator2")
  (return))

(fn `OnPlayerReachedApex`
  (`/Game/RoadToTemehani/Core/StateManager/AC_PlayerStatesManager.HandleStateTransition` (`self.GetPlayerStatesManager`) "NewEnumerator9")
  (return))