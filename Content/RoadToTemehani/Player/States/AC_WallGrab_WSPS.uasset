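; Player state for wall grabbing, available near a wall until the player is exhausted.
; Enter switches to custom movement, resizes the capsule and snaps the player to the wall; Exit restores falling and capsule size.
; A looping timer, paused between grabs and cleared on landing, drives tired flipbook and sound, then forces wall slide or fall.
; Input transitions to wall jump, or on release to ground locomotion, slide or fall.
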(event `self.ReceiveBeginPlay`
  ;[1 1 1] Each time the player touches the ground, we reset the chrono so the player can wall grab again
  (`parent.ReceiveBeginPlay`)
  (add `/Game/RoadToTemehani/Player/BP_Player.OnPlayerLanded` (`self.Player Actor`) (delegate `ClearFatigueTimer`)))

(event `ClearFatigueTimer`
  (params (Hit :type "HitResult Structure"))
  ;[1 1 1] Each time the player touches the ground, we reset the chrono so the player can wall grab again
  (`KismetSystemLibrary.K2_ClearAndInvalidateTimerHandle` (`self.GrabTimer`))
  (set `self.bCanWallGrab` true)
  (set `self.bTired` false))

(fn `Enter`
  (params (PreviousState :type "/Game/RoadToTemehani/Core/StateManager/EPlayerStates Enum" :default "NewEnumerator7"))
  (bind _flipbook_manager (`self.GetPlayerFlipbookManager`))
  (bind _capsulecomponent (`Character.CapsuleComponent` (`self.Player Actor`)))
  (`parent.Enter` PreviousState)
  (`CharacterMovementComponent.SetMovementMode` (`self.GetPlayerMovementComponent`) "MOVE_Custom" 0)
  ;[1 1 1] Resizes the player's capsule to stick him to the wall
  (set `self.DefaultCapsuleRadius` (`CapsuleComponent.CapsuleRadius` _capsulecomponent))
  (`CapsuleComponent.SetCapsuleRadius` _capsulecomponent (`self.TargetCapsuleRadius`) true)
  (`self.SnapPlayerToWall`)
  (`self.Orient Player for Wall Movement`)
  (`GameplayStatics.SpawnSound2D` (`self.WallGrabStartSFX`) 1.0 1.0 0.0 null)
  ;[1 1 1] We select different sound effects and animations depending on the fatigue state of the player
  (if (`self.bTired`)
    (`/Game/RoadToTemehani/Core/FlipbookManager/AC_FlipbookManager.PlayLoopingAnimation` _flipbook_manager (`self.WallGrabTiredFB`) "None")
    (bind _returnvalue (`GameplayStatics.SpawnSound2D` (`self.WallGrabTiredSFX`) 1.0 1.0 0.0 null))
    (set `self.AudioComponent` _returnvalue)
    (else
      (`/Game/RoadToTemehani/Core/FlipbookManager/AC_FlipbookManager.PlayLoopingAnimation` _flipbook_manager (`self.WallGrabIdleFB`) "None")))
  ;[1 1 1] If the timer is paused, we unpause it, else we create a new chrono
  (if (`KismetSystemLibrary.K2_IsTimerPausedHandle` (`self.GrabTimer`))
    (`KismetSystemLibrary.K2_UnPauseTimerHandle` (`self.GrabTimer`))
    (else
      (set `self.ElapsedTime` 0.0)
      (bind _returnvalue_2 (`KismetSystemLibrary.K2_SetTimerDelegate` (`|CreateDelegate` :!event `IncrementTime`) (`self.TimeStep`) true))
      (set `self.GrabTimer` _returnvalue_2)))
  (return))

(fn `Exit`
  (params (NextState :type "/Game/RoadToTemehani/Core/StateManager/EPlayerStates Enum" :default "NewEnumerator7"))
  (bind _grabtimer (`self.GrabTimer`))
  (`parent.Exit` NextState)
  (`CharacterMovementComponent.SetMovementMode` (`self.GetPlayerMovementComponent`) "MOVE_Falling" 0)
  (`CapsuleComponent.SetCapsuleRadius` (`Character.CapsuleComponent` (`self.Player Actor`)) (`self.DefaultCapsuleRadius`) true)
  (if (`KismetSystemLibrary.K2_IsTimerActiveHandle` _grabtimer)
    (`KismetSystemLibrary.K2_PauseTimerHandle` _grabtimer))
  ;[1 1 1] We stop playing the fatigue sounds, but only if they are playing
  (bind _audiocomponent (`self.AudioComponent`)
    (:`then`
      (`AudioComponent.Stop` _audiocomponent)
      (`self.K2_DestroyComponent` _audiocomponent))
    (:`else`
      _))
  (return))

(fn `HandleInput`
  (params (InputType :type "/Game/RoadToTemehani/Core/StateManager/EPlayerInputs Enum" :default "NewEnumerator1") (bPressed :type Boolean))
  (returns (bChangeState :type Boolean) (TargetState :type "/Game/RoadToTemehani/Core/StateManager/EPlayerStates Enum"))
  (bind _floorresult_bblockinghit (break `FindFloorResult` (`CharacterMovementComponent.K2_FindFloor` (`self.GetPlayerMovementComponent`) (`Actor.K2_GetActorLocation` (`self.Player Actor`)))))
  (`parent.HandleInput` InputType bPressed)
  ;[1 1 1] Handles Wall Jump
  (`/Game/RoadToTemehani/Core/StateManager/BPML_PlayerStatesUtilities.IsInputPressed?` InputType bPressed "NewEnumerator3"
    (:`Yes`
      (return true "NewEnumerator12"))
    (:`No`
      ;[1 1 1] Manages Wall Slide, Fall and Ground locomotion Transition
      (`/Game/RoadToTemehani/Core/StateManager/BPML_PlayerStatesUtilities.IsInputReleased?` InputType bPressed "NewEnumerator4"
        (:`Yes`
          (if _floorresult_bblockinghit
            (return true "NewEnumerator5")
            (elif (`self.IsPlayerMovingTowardsWall`)
              (return true "NewEnumerator13")
              (else
                (return true "NewEnumerator9")))))
        (:`No`
          (return false "NewEnumerator7"))))))

(fn `IncrementTime`
  (bind _output_get (set `self.ElapsedTime` (+ (`self.TimeStep`) (`self.ElapsedTime`))))
  (if (and (>= _output_get (`self.DurationBeforeTired`)) (not (`self.bTired`)))
    (set `self.bTired` true)
    (`/Game/RoadToTemehani/Core/FlipbookManager/AC_FlipbookManager.PlayLoopingAnimation` (`self.GetPlayerFlipbookManager`) (`self.WallGrabTiredFB`) "None")
    (bind _returnvalue (`GameplayStatics.SpawnSound2D` (`self.WallGrabTiredSFX`) 1.0 1.0 0.0 null))
    (set `self.AudioComponent` _returnvalue)
    (return)
    (elif (>= (`self.ElapsedTime`) (`self.DurationBeforeExhausted`))
      (set `self.bCanWallGrab` false)
      (`KismetSystemLibrary.K2_ClearAndInvalidateTimerHandle` (`self.GrabTimer`))
      (`/Game/RoadToTemehani/Core/StateManager/AC_PlayerStatesManager.SelectStateFromBool` (`self.GetPlayerStatesManager`) "NewEnumerator13" "NewEnumerator9" (`self.IsPlayerMovingTowardsWall`))
      (return)
      (else
        (return)))))

(fn `IsAccessible`
  (returns (bResult :type Boolean))
  ;[1 1 1] We can access the wall grab state only if the player still has the possibility to wall grab and is close to a wall
  (`parent.IsAccessible`)
  (bind _bwaswallfound (`self.UpdateWallProximityInfo`))
  (return (and _bwaswallfound (`self.bCanWallGrab`))))