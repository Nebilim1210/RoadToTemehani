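; Player state component for the rising phase of a jump in a flipbook-based character state machine.
; On enter it launches the player along trajectory parameters, plays jump animation and sound, and binds landed and apex events, unbinding on exit.
; Input drives air movement or switches to wall jump near walls, double jump otherwise, or glide.
; Reaching the apex moves to another state; landing early picks the next state from held input.
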(fn `Enter`
  (params (PreviousState :type "/Game/RoadToTemehani/Core/StateManager/EPlayerStates Enum" :default "NewEnumerator7"))
  (`parent.Enter` PreviousState)
  (add `/Game/RoadToTemehani/Player/BP_Player.OnPlayerLanded` (`self.Player Actor`) (`|CreateDelegate` :!event `OnPlayerLanded`))
  (add `Character.OnReachedJumpApex` (`self.Player Actor`) (`|CreateDelegate` :!event `OnPlayerReachedApex`))
  (set `CharacterMovementComponent.bNotifyApex` true (`self.GetPlayerMovementComponent`))
  (`/Game/RoadToTemehani/Player/BP_Player.Launch` (`self.Player Actor`) (`self.TrajectoryParameters`) (0.0 0.0 1.0) (0.0 0.0 0.0) false true)
  (`/Game/RoadToTemehani/Core/FlipbookManager/AC_FlipbookManager.PlayLoopingAnimation` (`self.GetPlayerFlipbookManager`) (`self.JumpUpFB`) "None")
  (`GameplayStatics.SpawnSound2D` (`self.JumpStartSfx`) 1.0 1.0 0.0 null)
  (return))

(fn `Exit`
  (params (NextState :type "/Game/RoadToTemehani/Core/StateManager/EPlayerStates Enum" :default "NewEnumerator7"))
  (bind _player_actor (`self.Player Actor`))
  (`parent.Exit` NextState)
  (remove `/Game/RoadToTemehani/Player/BP_Player.OnPlayerLanded` _player_actor (`|CreateDelegate` :!event `OnPlayerLanded`))
  (remove `Character.OnReachedJumpApex` _player_actor (`|CreateDelegate` :!event `OnPlayerReachedApex`))
  (set `CharacterMovementComponent.bNotifyApex` false (`self.GetPlayerMovementComponent`))
  (return))

(fn `HandleInput`
  (params (InputType :type "/Game/RoadToTemehani/Core/StateManager/EPlayerInputs Enum" :default "NewEnumerator1") (bPressed :type Boolean))
  (returns (bChangeState :type Boolean) (TargetState :type "/Game/RoadToTemehani/Core/StateManager/EPlayerStates Enum"))
  (`parent.HandleInput` InputType bPressed)
  ;[1 1 1] Handles Air horizontal movement
  (bind (_inputtypepassthrough _bpressedpassthrough) (`/Game/RoadToTemehani/Core/StateManager/BPML_PlayerStatesUtilities.IsInputEqualTo?` InputType bPressed)
    (:`Yes`
      (`self.Add Movement Input` _bpressedpassthrough)
      (return false "NewEnumerator7"))
    (:`No`
      ;[1 1 1] Handles Double Jump/Wall Jump
      (bind (_inputtypepassthrough_2 _bpressedpassthrough_2) (`/Game/RoadToTemehani/Core/StateManager/BPML_PlayerStatesUtilities.IsInputPressed?` InputType bPressed "NewEnumerator3")
        (:`Yes`
          (if (`self.IsPlayerCloseToA_Wall`)
            (return true "NewEnumerator12")
            (else
              (return true "NewEnumerator10"))))
        (:`No`
          ;[1 1 1] Handles Gliding Transition
          (`/Game/RoadToTemehani/Core/StateManager/BPML_PlayerStatesUtilities.IsInputPressed?` _inputtypepassthrough_2 _bpressedpassthrough_2 "NewEnumerator4"
            (:`Yes`
              (return true "NewEnumerator11"))
            (:`No`
              (return false "NewEnumerator7"))))))))

(fn `OnPlayerLanded`
  (params (Hit :type "HitResult Structure"))
  (`/Game/RoadToTemehani/Core/StateManager/AC_PlayerStatesManager.SelectStateFromInputPressed` (`self.GetPlayerStatesManager`) "NewEnumerator6" "NewEnumerator5" "NewEnumerator2")
  (return))

(fn `OnPlayerReachedApex`
  (`/Game/RoadToTemehani/Core/StateManager/AC_PlayerStatesManager.HandleStateTransition` (`self.GetPlayerStatesManager`) "NewEnumerator9")
  (return))