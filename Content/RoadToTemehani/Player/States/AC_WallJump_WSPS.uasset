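; Player state component for the wall jump, accessible only when a wall is nearby.
; On enter it zeroes velocity, orients the player and launches them away from the wall with sound and a start flipbook montage that leads into a looping jump animation.
; Bound landing and apex events pick the next state from held input.
; A specific input press near a wall requests a state change to chain wall jumps.
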(fn `Enter`
  (params (PreviousState :type "/Game/RoadToTemehani/Core/StateManager/EPlayerStates Enum" :default "NewEnumerator7"))
  (bind _player_actor (`self.Player Actor`))
  (`parent.Enter` PreviousState)
  (add `/Game/RoadToTemehani/Core/FlipbookManager/AC_FlipbookManager.OnAnimationPlaybackFinished` (`self.GetPlayerFlipbookManager`) (`|CreateDelegate` :!event `OnAnimMontageFinished`))
  (add `/Game/RoadToTemehani/Player/BP_Player.OnPlayerLanded` _player_actor (`|CreateDelegate` :!event `OnPlayerLanded`))
  (add `Character.OnReachedJumpApex` _player_actor (`|CreateDelegate` :!event `OnPlayerReachedApex`))
  (set `CharacterMovementComponent.bNotifyApex` true (`self.GetPlayerMovementComponent`))
  (`self.TriggerWallJump`)
  (return))

(fn `Exit`
  (params (NextState :type "/Game/RoadToTemehani/Core/StateManager/EPlayerStates Enum" :default "NewEnumerator7"))
  (bind _player_actor (`self.Player Actor`))
  (`parent.Exit` NextState)
  (remove `/Game/RoadToTemehani/Core/FlipbookManager/AC_FlipbookManager.OnAnimationPlaybackFinished` (`self.GetPlayerFlipbookManager`) (`|CreateDelegate` :!event `OnAnimMontageFinished`))
  (remove `Character.OnReachedJumpApex` _player_actor (`|CreateDelegate` :!event `OnPlayerReachedApex`))
  (remove `/Game/RoadToTemehani/Player/BP_Player.OnPlayerLanded` _player_actor (`|CreateDelegate` :!event `OnPlayerLanded`))
  (set `CharacterMovementComponent.bNotifyApex` false (`self.GetPlayerMovementComponent`))
  (return))

(fn `HandleInput`
  (params (InputType :type "/Game/RoadToTemehani/Core/StateManager/EPlayerInputs Enum" :default "NewEnumerator1") (bPressed :type Boolean))
  (returns (bChangeState :type Boolean) (TargetState :type "/Game/RoadToTemehani/Core/StateManager/EPlayerStates Enum"))
  (`parent.HandleInput` InputType bPressed)
  ;[1 1 1] Handles Wall Jump Chains
  (`/Game/RoadToTemehani/Core/StateManager/BPML_PlayerStatesUtilities.IsInputPressed?` InputType bPressed "NewEnumerator3"
    (:`Yes`
      (if (`self.IsPlayerCloseToA_Wall`)
        (return true "NewEnumerator12")
        (else
          _)))
    (:`No`
      _))
  (return false "NewEnumerator12"))

(fn `IsAccessible`
  (returns (bResult :type Boolean))
  ;[1 1 1] The player can only wall jump if there is a wall nearby.
  (`parent.IsAccessible`)
  (bind _bwaswallfound (`self.UpdateWallProximityInfo`))
  (return _bwaswallfound))

(fn `OnAnimMontageFinished`
  (params (Tag :type Name))
  ;[1 1 1] Plays the wall jump animation's second phase
  (if (== Tag "WallJumpStart")
    (`/Game/RoadToTemehani/Core/FlipbookManager/AC_FlipbookManager.PlayLoopingAnimation` (`self.GetPlayerFlipbookManager`) (`self.JumpUpLoopFB`) "None"))
  (return))

(fn `OnPlayerLanded`
  (params (Hit :type "HitResult Structure"))
  (`/Game/RoadToTemehani/Core/StateManager/AC_PlayerStatesManager.SelectStateFromInputPressed` (`self.GetPlayerStatesManager`) "NewEnumerator6" "NewEnumerator5" "NewEnumerator2")
  (return))

(fn `OnPlayerReachedApex`
  (`/Game/RoadToTemehani/Core/StateManager/AC_PlayerStatesManager.SelectStateFromInputPressed` (`self.GetPlayerStatesManager`) "NewEnumerator11" "NewEnumerator9" "NewEnumerator4")
  (return))

(fn `TriggerWallJump`
  (set `MovementComponent.Velocity` (0.0 0.0 0.0) (`self.GetPlayerMovementComponent`)) ; Disables the player's current velocity (not that useful, since\n we use Launch right after with XYZ override but hey it's safer)
  (`self.OrientPlayerForWallMovement`)
  (`/Game/RoadToTemehani/Player/BP_Player.Launch` (`self.Player Actor`) (`self.TrajectoryParameters`) (0.0 0.0 1.0) (`KismetMathLibrary.MakeVector` (* (`self.HorizontalImpulse`) (`self.GetWallOrientation`))) true true) ; Ejects the player in the airs
  (`/Game/RoadToTemehani/Core/FlipbookManager/AC_FlipbookManager.PlayMontage` (`self.GetPlayerFlipbookManager`) (`self.WallJumpStartFB`) "WallJumpStart")
  (`GameplayStatics.SpawnSound2D` (`self.WallJumpSFX`) 1.0 1.0 0.0 null)
  (return))