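; Player state component for wall sliding, entered only when wall proximity info confirms a nearby wall.
; Entering orients and snaps the player to the wall, cancels vertical velocity, swaps capsule radius and gravity, and starts looping slide animation and sound, with radius and sound cleaned up on exit.
; It falls when the player stops moving towards the wall, hands input to wall jump or wall grab, and picks a ground state from input on landing.
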(fn `Enter`
  (params (PreviousState :type "/Game/RoadToTemehani/Core/StateManager/EPlayerStates Enum" :default "NewEnumerator7"))
  (bind _capsulecomponent (`Character.CapsuleComponent` (`self.Player Actor`)))
  (`parent.Enter` PreviousState)
  (add `/Game/RoadToTemehani/Player/BP_Player.OnPlayerLanded` (`self.Player Actor`) (`|CreateDelegate` :!event `OnPlayerLanded`))
  (`self.Orient Player for Wall Movement`)
  (`self.StopPlayerVelocityZ`)
  (set `self.DefaultCapsuleRadius` (`CapsuleComponent.CapsuleRadius` _capsulecomponent)) ; Stores the player's capsule size when we enter the state.
  (`CapsuleComponent.SetCapsuleRadius` _capsulecomponent (`self.TargetCapsuleRadius`) true)
  (`self.SnapPlayerToWall`)
  (`/Game/RoadToTemehani/Player/BP_Player.UpdateGravityScale` (`self.Player Actor`) (`self.TrajectoryParameters`))
  (`self.StopPlayerVelocityZ`)
  (`/Game/RoadToTemehani/Core/FlipbookManager/AC_FlipbookManager.PlayLoopingAnimation` (`self.GetPlayerFlipbookManager`) (`self.WallSlideLoopFB`) "None")
  (bind _returnvalue (`GameplayStatics.SpawnSound2D` (`self.WallSlideLoopSFX`) 1.0 1.0 0.0 null false false))
  (set `self.AudioComponent` _returnvalue)
  (return))

(fn `Exit`
  (params (NextState :type "/Game/RoadToTemehani/Core/StateManager/EPlayerStates Enum" :default "NewEnumerator7"))
  (bind _audiocomponent (`self.AudioComponent`))
  (`parent.Exit` NextState)
  (remove `/Game/RoadToTemehani/Player/BP_Player.OnPlayerLanded` (`self.Player Actor`) (`|CreateDelegate` :!event `OnPlayerLanded`))
  (`AudioComponent.Stop` _audiocomponent)
  (`self.K2_DestroyComponent` _audiocomponent)
  (`CapsuleComponent.SetCapsuleRadius` (`Character.CapsuleComponent` (`self.Player Actor`)) (`self.DefaultCapsuleRadius`) true)
  (return))

(fn `HandleInput`
  (params (InputType :type "/Game/RoadToTemehani/Core/StateManager/EPlayerInputs Enum" :default "NewEnumerator1") (bPressed :type Boolean))
  (returns (bChangeState :type Boolean) (TargetState :type "/Game/RoadToTemehani/Core/StateManager/EPlayerStates Enum"))
  (`parent.HandleInput` InputType bPressed)
  ;[1 1 1] Manages Wall Jump
  (bind (_inputtypepassthrough _bpressedpassthrough) (`/Game/RoadToTemehani/Core/StateManager/BPML_PlayerStatesUtilities.IsInputPressed?` InputType bPressed "NewEnumerator3")
    (:`Yes`
      (return true "NewEnumerator12"))
    (:`No`
      ;[1 1 1] Manages Wall Grab Transition
      (`/Game/RoadToTemehani/Core/StateManager/BPML_PlayerStatesUtilities.IsInputPressed?` _inputtypepassthrough _bpressedpassthrough "NewEnumerator4"
        (:`Yes`
          (return true "NewEnumerator14"))
        (:`No`
          (return false "NewEnumerator7"))))))

(fn `IsAccessible`
  (returns (bResult :type Boolean))
  (`parent.IsAccessible`)
  (bind _bwaswallfound (`self.UpdateWallProximityInfo`))
  (return _bwaswallfound))

(fn `OnPlayerLanded`
  (params (Hit :type "HitResult Structure"))
  (`/Game/RoadToTemehani/Core/StateManager/AC_PlayerStatesManager.SelectStateFromInputPressed` (`self.GetPlayerStatesManager`) "NewEnumerator6" "NewEnumerator5" "NewEnumerator2")
  (return))

(fn `StopPlayerVelocityZ`
  (bind _character_movement (`self.GetPlayerMovementComponent`))
  (bind (_velocity_x _velocity_y) (`KismetMathLibrary.BreakVector` (`MovementComponent.Velocity` _character_movement)))
  (set `MovementComponent.Velocity` (`KismetMathLibrary.MakeVector` _velocity_x _velocity_y) _character_movement)
  (return))

(fn `Update`
  ;[1 1 1] As soon as the player doesn't tilt his stick towards the wall, or if there is no wall anymore, we go to the state fall.
  (`parent.Update`)
  (if (not (`self.IsPlayerMovingTowardsWall`))
    (`/Game/RoadToTemehani/Core/StateManager/AC_PlayerStatesManager.HandleStateTransition` (`self.GetPlayerStatesManager`) "NewEnumerator9"))
  (return))