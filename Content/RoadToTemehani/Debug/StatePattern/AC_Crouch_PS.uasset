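; AC_Crouch_PS is the crouch state in the player's state-pattern implementation.
; Enter and Exit run the parent logic, then call StartCrouch and StopCrouch on the owning BP_Player.
; HandleInput compares incoming input against one input type and requests a transition to another state only when that input is released, so crouch works as a hold action.
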(fn `Enter`
  (params (PreviousState :type "/Game/RoadToTemehani/Core/StateManager/EPlayerStates Enum" :default "NewEnumerator5"))
  (`parent.Enter` PreviousState)
  (bind _asbp_player (cast `/Game/RoadToTemehani/Debug/StatePattern/BP_Player` (`self.GetOwner`)))
  (`/Game/RoadToTemehani/Debug/StatePattern/BP_Player.StartCrouch` _asbp_player)
  (return))

(fn `Exit`
  (params (NextState :type "/Game/RoadToTemehani/Core/StateManager/EPlayerStates Enum" :default "NewEnumerator5"))
  (`parent.Exit` NextState)
  (bind _asbp_player (cast `/Game/RoadToTemehani/Debug/StatePattern/BP_Player` (`self.GetOwner`)))
  (`/Game/RoadToTemehani/Debug/StatePattern/BP_Player.StopCrouch` _asbp_player))

(fn `HandleInput`
  (params (InputType :type "/Game/RoadToTemehani/Core/StateManager/EPlayerInputs Enum" :default "NewEnumerator1") (bPressed :type Boolean))
  (returns (bChangeState :type Boolean) (TargetState :type "/Game/RoadToTemehani/Core/StateManager/EPlayerStates Enum"))
  (`parent.HandleInput` InputType bPressed)
  (`/Game/RoadToTemehani/Core/StateManager/BPML_PlayerStatesUtilities.CompareInputEventTo` InputType bPressed "NewEnumerator1"
    (:`Pressed`
      _)
    (:`Released`
      (return true "NewEnumerator5"))
    (:`Unused`
      _))
  (return false "NewEnumerator5"))