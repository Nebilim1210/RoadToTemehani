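; Debug player character that demonstrates a simple state machine with Idle, Jump, Crouch and Dive states.
; Space and Left Ctrl trigger transitions based on CurrentState: jump from Idle, crouch while held from Idle, or dive from Jump; landing returns to Idle.
; Jump and dive use vertical launches, crouch shrinks and lowers the Sphere, and ChangeColor tints it per state through a newly created dynamic material.
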(event `self.OnLanded`
  (params (Hit :type "HitResult Structure (by ref)"))
  (`self.ChangeColor` "NewEnumerator0")
  (set `self.CurrentState` "NewEnumerator0"))

(event `Key|SpaceBar`
  (params (Key :type "Key Structure"))
  (:`Pressed`
    (if (`|EnumEquality` (`self.CurrentState`) "NewEnumerator0")
      (`self.StartJump`)
      (set `self.CurrentState` "NewEnumerator1"))))

(event `Key|LeftControl`
  (params (Key :type "Key Structure"))
  (:`Pressed`
    (switch `/Game/RoadToTemehani/Debug/StatePattern/EState` (`self.CurrentState`)
      (:`NewEnumerator0`
        (`self.StartCrouch`)
        (set `self.CurrentState` "NewEnumerator2"))
      (:`NewEnumerator1`
        (`self.StartDive`)
        (set `self.CurrentState` "NewEnumerator3"))))
  (:`Released`
    (if (`|EnumEquality` (`self.CurrentState`) "NewEnumerator2")
      (`self.StopCrouch`)
      (set `self.CurrentState` "NewEnumerator0"))))

(fn `ChangeColor`
  (params (State :type "/Game/RoadToTemehani/Debug/StatePattern/EState Enum" :default "NewEnumerator0"))
  (bind _returnvalue (`PrimitiveComponent.CreateDynamicMaterialInstance` (`self.Sphere`) 0 null "None"))
  (`MaterialInstanceDynamic.SetVectorParameterValue` _returnvalue "Color" (select `/Game/RoadToTemehani/Debug/StatePattern/EState` State :`NewEnumerator0` (struct :`G` 0.370958 :`B` 1.0 :`A` 1.0) :`NewEnumerator1` (struct :`R` 0.078221 :`G` 1.0 :`A` 1.0) :`NewEnumerator2` (struct :`R` 1.0 :`G` 0.883522 :`A` 1.0) :`NewEnumerator3` (struct :`R` 1.0 :`B` 0.829009 :`A` 1.0) :!type "LinearColor Structure")))

(fn `StartCrouch`
  (`SceneComponent.K2_SetRelativeTransform` (`self.Sphere`) (`KismetMathLibrary.MakeTransform` (0.0 0.0 -15.0) (struct) (0.7 0.7 0.7)) false true)
  (`self.ChangeColor` "NewEnumerator2"))

(fn `StartDive`
  (`self.LaunchCharacter` (0.0 0.0 -1500.0) false true)
  (`self.ChangeColor` "NewEnumerator3"))

(fn `StartJump`
  (`self.LaunchCharacter` (0.0 0.0 800.0) false true)
  (`self.ChangeColor` "NewEnumerator1"))

(fn `StopCrouch`
  (`SceneComponent.K2_SetRelativeTransform` (`self.Sphere`) (`KismetMathLibrary.MakeTransform` (0.0 0.0 0.0)) false true)
  (`self.ChangeColor` "NewEnumerator0"))

(fn `UserConstructionScript`
  (`self.ChangeColor` "NewEnumerator0"))