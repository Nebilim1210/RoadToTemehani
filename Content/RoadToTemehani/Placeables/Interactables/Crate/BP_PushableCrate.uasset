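; Pushable crate that stays non-physical while grounded and falls under physics when it loses its support.
; TryToTriggerFalling casts three short downward traces along the bottom X extent, enables physics only if all miss, and returns whether it falls.
; When the box goes to sleep, physics switches off again so only the pushing mechanism can move it.
; While falling, upward-facing non-player hits play a landing sound if the impulse is large relative to mass.
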(event `self.Box.OnComponentSleep`
  (params (SleepingComponent :type "PrimitiveComponent Object Reference") (BoneName :type Name))
  ;[1 1 1] After the crate stayed grounded long enough, we disable its physics to allow its movements only if the player activates the crate pushing mechanism
  (`PrimitiveComponent.SetSimulatePhysics` SleepingComponent false))

(event `self.Box.OnComponentHit`
  (params (HitComponent :type "PrimitiveComponent Object Reference") (OtherActor :type "Actor Object Reference") (OtherComp :type "PrimitiveComponent Object Reference") (NormalImpulse :type "Vector Structure") (Hit :type "HitResult Structure (by ref)"))
  ;[1 1 1] We play the crate falling sound effect only if it's hitting the ground, at a fast enought speed
  (if (and (`SceneComponent.IsSimulatingPhysics` (`self.Box`) "None") (!= OtherActor (`GameplayStatics.GetPlayerPawn` 0)) (> (`KismetMathLibrary.Dot_VectorVector` (`KismetMathLibrary.Normal` NormalImpulse) (0.0 0.0 1.0)) 0.9))
    (if (> (/ (.z NormalImpulse) 1000.0) (* (`PrimitiveComponent.GetMass` (`self.Box`)) 0.3))
      (`GameplayStatics.SpawnSoundAtLocation` (`self.HitGroundSFX`) (`self.K2_GetActorLocation`) (struct) 1.0 1.0 0.0 null null))))

(fn `TryToTriggerFalling`
  (returns (bSuccess :type Boolean))
  (locals (L_TraesSpacing :type "Float (double-precision)" :default 0.0) (L_BottomLeftCornerLoc :type "Vector Structure"))
  (bind (_returnvalue_x _returnvalue_y _returnvalue_z) (`KismetMathLibrary.BreakVector` (`BoxComponent.GetScaledBoxExtent` (`self.Box`))))
  (set `local.L_TraesSpacing` _returnvalue_x) ; Spacing between rays.
  (set `local.L_BottomLeftCornerLoc` (- (`self.K2_GetActorLocation`) (`KismetMathLibrary.MakeVector` _returnvalue_x 0.0 _returnvalue_z))) ; Bottom left corner of the crate
  (for _index (range 3)
    (bind _returnvalue (+ (`local.L_BottomLeftCornerLoc`) (`KismetMathLibrary.MakeVector` (* _index (`local.L_TraesSpacing`)))))
    (bind (_outhit _returnvalue_2) (`KismetSystemLibrary.LineTraceSingleByProfile` _returnvalue (- _returnvalue (`KismetMathLibrary.MakeVector` 0.0 0.0 (`self.FloorSearchDistance`))) "Pawn"))
    (if _returnvalue_2
      (return false)))
  (`PrimitiveComponent.SetSimulatePhysics` (`self.Box`) true) ; No ray has touched the ground, so we activate the physics to make the crate fall.
  (return true))

(fn `UserConstructionScript`)