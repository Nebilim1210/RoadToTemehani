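; Actor component that takes over the owner's Paper Flipbook component to manage 2D sprite animation playback.
; It disables native playback and steps frames with a looping timer at the flipbook's framerate, supporting play, pause, stop, looping, tagged switching and restartable montages.
; Each step fires dispatchers for loop or finish, plus opt-in tracking of chosen frames and sockets, acting as animation notifies reset on animation change.
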(event `self.ReceiveBeginPlay`
  (bind _bissystemvalid (`self.InitializeSystem`))
  (if (and _bissystemvalid (`self.bAutoStart`))
    (`self.Play` (`self.bShouldLoop`))))

(fn `CheckIfFrameIsTracked`
  (params (`Frame Index` :type Integer))
  (bind _returnvalue (- `Frame Index` 1))
  (if (`KismetArrayLibrary.Array_Contains` (`self.FramesToTrack`) _returnvalue)
    (`self.OnTrackedFrameFound` _returnvalue))
  (return))

(fn `CheckIfSocketIsTracked`
  (params (SocketFrameIndex :type Integer))
  (bind _returnvalue (- SocketFrameIndex 1))
  (if (`KismetArrayLibrary.Array_Contains` (`self.SocketsToTrackIndexes`) _returnvalue)
    ;[1 1 1] Multiple sockets might be placed on the same frame. So rather than returning the first occurence of the current index, we go through the whole array to find every socket defined in a same frame
    (for (_array_element _array_index) (`self.SocketsToTrackIndexes`)
      (if (== _array_element _returnvalue)
        (bind _output (`|GetArrayItem` (`self.SocketsNamesToTrack`) _array_index))
        (`self.OnTrackedSocketFound` _output _returnvalue (`self.GetSocketLocation` _output)))))
  (return))

(fn `GetCurrentFrameIndex`
  (returns (CurrentFrame :type Integer))
  (`self.IsSystemValid`
    (:`Yes`
      (return (- (`self.CurrentFrameIndex`) 1)))
    (:`No`
      (return -1))))

(fn `GetCurrentFrameInfo`
  (returns (CurrentFrameIndex :type Integer) (CurrentFrameSprite :type "PaperSprite Object Reference"))
  (bind _currentframeindex (`self.CurrentFrameIndex`))
  (`self.IsSystemValid`
    (:`Yes`
      (return _currentframeindex (`PaperFlipbook.GetSpriteAtFrame` (`PaperFlipbookComponent.GetFlipbook` (`self.OwnerPaperFlipbookComponent`)) _currentframeindex)))
    (:`No`
      (return -1 null))))

(fn `GetCurrentTag`
  (returns (CurrentTag :type Name))
  (`self.IsSystemValid`
    (:`Yes`
      (return (`self.CurrentTag`)))
    (:`No`
      (return "None"))))

(fn `GetFlipbook`
  (returns (ReturnValue :type "PaperFlipbook Object Reference"))
  (`self.IsSystemValid`
    (:`Yes`
      (return (`PaperFlipbookComponent.GetFlipbook` (`self.OwnerPaperFlipbookComponent`))))
    (:`No`
      (return null))))

(fn `GetSocketLocation`
  (params (InSocketName :type Name))
  (returns (ReturnValue :type "Vector Structure"))
  (return (`SceneComponent.GetSocketLocation` (`self.OwnerPaperFlipbookComponent`) InSocketName)))

(fn `IncrementPlayback`
  (bind _currentframeindex (`self.CurrentFrameIndex`))
  (bind _currenttag (`self.CurrentTag`))
  (`PaperFlipbookComponent.SetPlaybackPositionInFrames` (`self.OwnerPaperFlipbookComponent`) _currentframeindex false) ; Displays current frame
  (`self.OnCheckFrameTracked` _currentframeindex)
  (`self.OnCheckSocketTracked` _currentframeindex)
  (if (< _currentframeindex (`self.MaxNumFrames`))
    (`/Engine/EditorBlueprintResources/StandardMacros.IncrementInt` (`self.CurrentFrameIndex`)
      (:`  `
        _))
    (elif (`self.bShouldLoop`)
      (set `self.CurrentFrameIndex` 1)
      (`self.OnLastFrameReachedWhileLooping` _currenttag)
      (else
        (`self.Pause`)
        (`self.OnAnimationPlaybackFinished` _currenttag))))
  (return))

(fn `InitializeSystem`
  (returns (bIsSystemValid :type Boolean))
  (bind _returnvalue (`self.GetOwner`))
  (bind _ownerpaperflipbookcomponent (`self.OwnerPaperFlipbookComponent`))
  (bind _returnvalue_2 (`Actor.GetComponentByClass` _returnvalue "/Script/Paper2D.PaperFlipbookComponent"))
  ;[0 0 0] Verifies if the owner posesses a flipbook Component. If he doesn't, the system is unusable
  (bind _output_get (set `self.bValid` (`KismetSystemLibrary.IsValid` _returnvalue_2)))
  (if _output_get
    (set `self.OwnerPaperFlipbookComponent` _returnvalue_2)
    ;[1 1 1] Sends a warning if we forgot to assign a flipbook asset to the paper flipbook component of the owner
    (`/Engine/EditorBlueprintResources/StandardMacros.IsValid` (`PaperFlipbookComponent.GetFlipbook` (`self.OwnerPaperFlipbookComponent`))
      (:`Is Valid`
        ;[1 1 1] On désactive tout chez le flipbook du owner et on remet la tête de lecture au début car c'est ce component qui va tout gérer
        (`PaperFlipbookComponent.SetLooping` _ownerpaperflipbookcomponent false)
        (`PaperFlipbookComponent.Stop` _ownerpaperflipbookcomponent)
        (`PaperFlipbookComponent.SetPlaybackPositionInFrames` _ownerpaperflipbookcomponent 1 false)
        (set `self.MaxNumFrames` (`PaperFlipbookComponent.GetFlipbookLengthInFrames` (`self.OwnerPaperFlipbookComponent`)))
        (set `self.CurrentFrameIndex` 1)
        (return true))
      (:`Is Not Valid`
        (`KismetSystemLibrary.PrintString` "Paper Flipbook component exists but doesn't have an assigned Flipbook asset" true true (struct :`R` 1.0 :`A` 1.0) 10.0)))
    (else
      (`KismetSystemLibrary.PrintString` (`KismetStringLibrary.Concat_StrStr` (`KismetSystemLibrary.GetDisplayName` _returnvalue) ": The flipbook manager component is assigned to an actor that has no paper flipbook component") true true (struct :`R` 1.0 :`A` 1.0) 10.0)
      (return false))))

(fn `IsTrackingFrames`
  (returns (bTrackingFrames :type Boolean))
  (return (`self.bTrackingFrames`)))

(fn `IsTrackingSockets`
  (returns (bTrackingSockets :type Boolean))
  (return (`self.bTrackingSockets`)))

(fn `Pause`
  (`self.IsSystemValid`
    (:`Yes`
      (if (`|EnumEquality` (`self.CurrentPlaybackState`) "NewEnumerator0")
        (`KismetSystemLibrary.K2_PauseTimerHandle` (`self.PlaybackTimer`))
        (set `self.CurrentPlaybackState` "NewEnumerator2")
        (return)
        (else
          _)))
    (:`No`
      _))
  (return))

(fn `Play`
  (params (bShouldLoop :type Boolean))
  (`self.IsSystemValid`
    (:`Yes`
      (set `self.bShouldLoop` bShouldLoop)
      (switch `/Game/RoadToTemehani/Core/FlipbookManager/E_FlipbookManagerState` (`self.CurrentPlaybackState`)
        (:`NewEnumerator0`
          (return) ; If the playback is already playing, do nothing
        )
        (:`NewEnumerator1`
          (if (> (`self.MaxNumFrames`) 1)
            (set `self.CurrentPlaybackState` "NewEnumerator0")
            (`self.IncrementPlayback`) ; Immediately displays the 1st frame
            (bind _returnvalue (`KismetSystemLibrary.K2_SetTimerDelegate` (`|CreateDelegate` :!event `IncrementPlayback`) (/ 1.0 (`PaperFlipbookComponent.GetFlipbookFramerate` (`self.OwnerPaperFlipbookComponent`))) true)) ; Displays the rest of the frames regularly
            (set `self.PlaybackTimer` _returnvalue)
            (return)))
        (:`NewEnumerator2`
          (set `self.CurrentPlaybackState` "NewEnumerator0")
          (`KismetSystemLibrary.K2_UnPauseTimerHandle` (`self.PlaybackTimer`))
          (return))))
    (:`No`
      (return))))

(fn `PlayAnimation`
  (params (NewFlipbook :type "PaperFlipbook Object Reference") (NewTag :type Name :default "None") (bShouldLoop :type Boolean) (bOverrideCurrentAnimation :type Boolean))
  (returns (Success :type Boolean))
  (`self.IsSystemValid`
    (:`Yes`
      (bind _wasflipbookchanged (`self.SetFlipbook` NewFlipbook NewTag))
      (if _wasflipbookchanged
        _
        (elif bOverrideCurrentAnimation
          ;[1 1 1] Stops the tracking systems when launching a new animation
          (`self.StopTrackingSockets`)
          (`self.StopTrackingFrames`)
          (else
            (return false))))
      (`self.PlayFromStart` bShouldLoop)
      (return true))
    (:`No`
      (return false))))

(fn `PlayAnimationAndTrackFrames`
  (params (NewFlipbook :type "PaperFlipbook Object Reference") (NewTag :type Name :default "None") (bShouldLoop :type Boolean) (bOverrideCurrentAnimation :type Boolean) (FramesToTrack :type "Array of Integer (by ref)"))
  (returns (Success :type Boolean))
  (bind _success (`self.PlayAnimation` NewFlipbook NewTag bShouldLoop bOverrideCurrentAnimation))
  (if _success
    (`self.StartTrackingFrames` FramesToTrack))
  (return _success))

(fn `PlayAnimationAndTrackSockets`
  (params (NewFlipbook :type "PaperFlipbook Object Reference") (NewTag :type Name :default "None") (bShouldLoop :type Boolean) (bOverrideCurrentAnimation :type Boolean) (SocketsNamesToTrack :type "Array of Name (by ref)") (SocketsToTrackIndexes :type "Array of Integer (by ref)"))
  (returns (Success :type Boolean))
  (bind _success (`self.PlayAnimation` NewFlipbook NewTag bShouldLoop bOverrideCurrentAnimation))
  (if _success
    (`self.StartTrackingSockets` SocketsNamesToTrack SocketsToTrackIndexes))
  (return _success))

(fn `PlayFromStart`
  (params (bShouldLoop :type Boolean))
  (`self.IsSystemValid`
    (:`Yes`
      (`self.Stop`)
      (`self.Play` bShouldLoop))
    (:`No`
      (return))))

(fn `PlayLoopingAnimation`
  (params (NewFlipbook :type "PaperFlipbook Object Reference") (NewTag :type Name))
  (returns (Success :type Boolean))
  (bind _success (`self.PlayAnimation` NewFlipbook NewTag true))
  (return _success))

(fn `PlayLoopingAnimationAndTrackFrames`
  (params (NewFlipbook :type "PaperFlipbook Object Reference") (NewTag :type Name :default "None") (FramesToTrack :type "Array of Integer (by ref)"))
  (returns (Success :type Boolean))
  (bind _success (`self.PlayLoopingAnimation` NewFlipbook NewTag))
  (if _success
    (`self.StartTrackingFrames` FramesToTrack))
  (return _success))

(fn `PlayLoopingAnimationAndTrackSockets`
  (params (NewFlipbook :type "PaperFlipbook Object Reference") (NewTag :type Name :default "None") (SocketsNamesToTrack :type "Array of Name (by ref)") (SocketsToTrackIndexes :type "Array of Integer (by ref)"))
  (returns (Success :type Boolean))
  (bind _success (`self.PlayLoopingAnimation` NewFlipbook NewTag))
  (if _success
    (`self.StartTrackingSockets` SocketsNamesToTrack SocketsToTrackIndexes))
  (return _success))

(fn `PlayMontage`
  (params (NewFlipbook :type "PaperFlipbook Object Reference") (NewTag :type Name))
  (returns (Success :type Boolean))
  (bind _success (`self.PlayAnimation` NewFlipbook NewTag false true))
  (return _success))

(fn `PlayMontageAndTrackFrames`
  (params (NewFlipbook :type "PaperFlipbook Object Reference") (NewTag :type Name :default "None") (FramesToTrack :type "Array of Integer (by ref)"))
  (returns (Success :type Boolean))
  (bind _success (`self.PlayMontage` NewFlipbook NewTag))
  (if _success
    (`self.StartTrackingFrames` FramesToTrack))
  (return _success))

(fn `PlayMontageAndTrackSockets`
  (params (NewFlipbook :type "PaperFlipbook Object Reference") (NewTag :type Name :default "None") (SocketsNamesToTrack :type "Array of Name (by ref)") (SocketsToTrackIndexes :type "Array of Integer (by ref)"))
  (returns (Success :type Boolean))
  (bind _success (`self.PlayMontage` NewFlipbook NewTag))
  (if _success
    (`self.StartTrackingSockets` SocketsNamesToTrack SocketsToTrackIndexes)
    (return _success)))

(fn `SetFlipbook`
  (params (NewFlipbook :type "PaperFlipbook Object Reference") (NewTag :type Name :default "None"))
  (returns (WasFlipbookChanged :type Boolean))
  (bind _ownerpaperflipbookcomponent (`self.OwnerPaperFlipbookComponent`))
  (`self.IsSystemValid`
    (:`Yes`
      (if (!= NewFlipbook (`PaperFlipbookComponent.GetFlipbook` _ownerpaperflipbookcomponent))
        (set `self.CurrentTag` NewTag)
        (`PaperFlipbookComponent.SetFlipbook` _ownerpaperflipbookcomponent NewFlipbook)
        (set `self.MaxNumFrames` (`PaperFlipbook.GetNumFrames` NewFlipbook))
        (`self.PlayFromStart` (`self.bShouldLoop`))
        ;[1 1 1] Stops the tracking systems when launching a new animation
        (`self.StopTrackingSockets`)
        (`self.StopTrackingFrames`)
        (return true)
        (else
          (return false))))
    (:`No`
      (return false))))

(fn `SetFlipbookAndTrackFrames`
  (params (NewFlipbook :type "PaperFlipbook Object Reference") (NewTag :type Name :default "None") (FramesToTrack :type "Array of Integer (by ref)"))
  (returns (WasFlipbookChanged :type Boolean))
  (bind _wasflipbookchanged (`self.SetFlipbook` NewFlipbook NewTag))
  (if _wasflipbookchanged
    (`self.StartTrackingFrames` FramesToTrack))
  (return _wasflipbookchanged))

(fn `SetFlipbookAndTrackSockets`
  (params (NewFlipbook :type "PaperFlipbook Object Reference") (NewTag :type Name :default "None") (SocketsNamesToTrack :type "Array of Name (by ref)") (SocketsToTrackIndexes :type "Array of Integer (by ref)"))
  (returns (WasFlipbookChanged :type Boolean))
  (bind _wasflipbookchanged (`self.SetFlipbook` NewFlipbook NewTag))
  (if _wasflipbookchanged
    (`self.StartTrackingSockets` SocketsNamesToTrack SocketsToTrackIndexes))
  (return _wasflipbookchanged))

(fn `SetLooping`
  (params (NewLooping :type Boolean))
  (set `self.bShouldLoop` NewLooping)
  (return))

(fn `StartTrackingFrames`
  (params (FramesToTrack :type "Array of Integer"))
  (`self.IsSystemValid`
    (:`Yes`
      (`self.StopTrackingFrames`)
      (set `self.FramesToTrack` FramesToTrack)
      (add `self.OnCheckFrameTracked` (`|CreateDelegate` :!event `CheckIfFrameIsTracked`))
      (set `self.bTrackingFrames` true))
    (:`No`
      _))
  (return))

(fn `StartTrackingSockets`
  (params (SocketsNamesToTrack :type "Array of Name") (SocketsToTrackIndexes :type "Array of Integer"))
  (`self.IsSystemValid`
    (:`Yes`
      (if (== (`KismetArrayLibrary.Array_Length` SocketsNamesToTrack) (`KismetArrayLibrary.Array_Length` SocketsToTrackIndexes))
        (`self.StopTrackingSockets`)
        (set `self.SocketsNamesToTrack` SocketsNamesToTrack)
        (set `self.SocketsToTrackIndexes` SocketsToTrackIndexes)
        (add `self.OnCheckSocketTracked` (`|CreateDelegate` :!event `CheckIfSocketIsTracked`))
        (set `self.bTrackingSockets` true)
        (else
          (`KismetSystemLibrary.PrintString` (`KismetStringLibrary.Concat_StrStr` (`KismetSystemLibrary.GetDisplayName` (`self.GetOwner`)) " : le tableau des sockets à traquer doit avoir la même taille que celui des frames à traquer !"))))
      (return))
    (:`No`
      (return))))

(fn `Stop`
  (`self.IsSystemValid`
    (:`Yes`
      (if (`|EnumInequality` (`self.CurrentPlaybackState`) "NewEnumerator1")
        (set `self.CurrentPlaybackState` "NewEnumerator1")
        (`KismetSystemLibrary.K2_ClearAndInvalidateTimerHandle` (`self.PlaybackTimer`))
        (bind _output_get (set `self.CurrentFrameIndex` 1))
        (`PaperFlipbookComponent.SetPlaybackPositionInFrames` (`self.OwnerPaperFlipbookComponent`) _output_get false)
        (return)
        (else
          _)))
    (:`No`
      _))
  (return))

(fn `StopTrackingFrames`
  (`self.IsSystemValid`
    (:`Yes`
      (if (`self.bTrackingFrames`)
        (`KismetArrayLibrary.Array_Clear` (`self.FramesToTrack`))
        (remove `self.OnCheckFrameTracked` (`|CreateDelegate` :!event `CheckIfFrameIsTracked`))
        (set `self.bTrackingFrames` false)))
    (:`No`
      _))
  (return))

(fn `StopTrackingSockets`
  (`self.IsSystemValid`
    (:`Yes`
      (if (`self.bTrackingSockets`)
        (`KismetArrayLibrary.Array_Clear` (`self.SocketsNamesToTrack`))
        (`KismetArrayLibrary.Array_Clear` (`self.SocketsToTrackIndexes`))
        (remove `self.OnCheckSocketTracked` (`|CreateDelegate` :!event `CheckIfSocketIsTracked`))
        (set `self.bTrackingSockets` false)))
    (:`No`
      _))
  (return))