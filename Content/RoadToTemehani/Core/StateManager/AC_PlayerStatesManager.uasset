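; AC_PlayerStatesManager is an actor component that runs the player's state machine, with each state as its own component.
; State components are created on demand from classes in a data asset, added to the owner and cached in a map.
; Transitions check accessibility, then call Exit and Enter, or notify the active state on failure.
; It also tracks pressed inputs and forwards them to the active state, which can request a transition.
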(fn `CallActiveStateUpdateFunction`
  (`/Game/RoadToTemehani/Core/StateManager/AC_PlayerState_Master.Update` (`self.ActiveState`))
  (return))

(fn `GetStateActorComponent`
  (params (StateType :type "/Game/RoadToTemehani/Core/StateManager/EPlayerStates Enum" :default "NewEnumerator0"))
  (returns (StateActorComponent :type "/Game/RoadToTemehani/Core/StateManager/AC_PlayerState_Master Object Reference"))
  (bind (_value _returnvalue) (`BlueprintMapLibrary.Map_Find` (`self.PlayerStateComponents`) StateType))
  ;[1 1 1] If the state has already been created, we get it from our map
  (if _returnvalue
    (return _value)
    (else
      ;[1 1 1] If the state has not been created yet, we create it, add it to the map of the states, and to the player.
      (bind _playerstateclassesdb (`self.PlayerStateClassesDB`)
        (:`then`
          (bind (_bfound _class) (`/Game/RoadToTemehani/Core/StateManager/DA_PlayerStateClasses.Get Player State Class` _playerstateclassesdb StateType))
          (if _bfound
            (bind _returnvalue_2 (`|AddComponentByClass` (`self.GetOwner`) _class))
            (`BlueprintMapLibrary.Map_Add` (`self.PlayerStateComponents`) StateType _returnvalue_2)
            (return _returnvalue_2)
            (else
              (`KismetSystemLibrary.PrintString` (`KismetStringLibrary.Concat_StrStr` "AC_PlayerStatesManager :No corresponding class to the type " (`|GetEnumeratorNameAsString` StateType) "exists in the Data Asset" (`KismetSystemLibrary.GetDisplayName` (`self.PlayerStateClassesDB`))) true true (struct :`R` 1.0 :`A` 1.0) 5.0)
              (return null))))
        (:`else`
          (`KismetSystemLibrary.PrintString` "AC_PlayerStatesManager has no data asset assigned" true true (struct :`R` 1.0 :`A` 1.0) 5.0)
          (return null))))))

(fn `HandlePlayerInput`
  (params (InputType :type "/Game/RoadToTemehani/Core/StateManager/EPlayerInputs Enum" :default "NewEnumerator1") (bPressed :type Boolean))
  (`self.UpdateCurrentInputsState` InputType bPressed) ; Updates the input state to keep track\nof which inputs are being pressed
  ;[1 1 1] Sends the input event to the the state, and if it correspond to a transition to another state, we launch the transition
  (bind (_bchangestate _targetstate) (`/Game/RoadToTemehani/Core/StateManager/AC_PlayerState_Master.HandleInput` (`self.ActiveState`) InputType bPressed))
  (if _bchangestate
    (`self.HandleStateTransition` _targetstate))
  (return))

(fn `HandleStateTransition`
  (params (TargetState :type "/Game/RoadToTemehani/Core/StateManager/EPlayerStates Enum" :default "NewEnumerator5"))
  (locals (L_NewStateType :type "/Game/RoadToTemehani/Core/StateManager/EPlayerStates Enum" :default "NewEnumerator5") (L_NewStateComponent :type "/Game/RoadToTemehani/Core/StateManager/AC_PlayerState_Master Object Reference"))
  (bind _output_get (set `local.L_NewStateType` TargetState))
  ;[1 1 1] Gets the state towards which we want to transition. If the actor component doesn't exist, it will be created in the function.
  (bind _stateactorcomponent (`self.GetStateActorComponent` _output_get))
  (bind _output_get_2 (set `local.L_NewStateComponent` _stateactorcomponent))
  (`/Engine/EditorBlueprintResources/StandardMacros.IsValid` _output_get_2 ; This Is valid will fail if the required state\nis not in the Data Asset.
    (:`Is Valid`
      ;[1 1 1] Checks if all conditions are met to access the state
      (bind _bresult (`/Game/RoadToTemehani/Core/StateManager/AC_PlayerState_Master.IsAccessible` _output_get_2))
      (if _bresult
        ;[1 1 1] If everything is okay, we call the Exit function of the active state, and the Enter function of the following one.
        (`|ExecutionSequence`
          (:`then_0`
            (bind _activestate (`self.ActiveState`)
              (:`then`
                (`/Game/RoadToTemehani/Core/StateManager/AC_PlayerState_Master.Exit` _activestate (`local.L_NewStateType`)))
              (:`else`)))
          (:`then_1`
            (bind _output_get_3 (set `self.ActiveState` (`local.L_NewStateComponent`)))
            (`/Game/RoadToTemehani/Core/StateManager/AC_PlayerState_Master.Enter` _output_get_3 (`self.ActiveStateName`))
            (set `self.ActiveStateName` (`local.L_NewStateType`))
            (return)))
        (else
          ;[1 1 1] If the new state is not accessible or it doesn't exist, we tell the active state we couldn't change state
          (bind _activestate_2 (`self.ActiveState` :!label _label)
            (:`then`
              (`/Game/RoadToTemehani/Core/StateManager/AC_PlayerState_Master.OnFailedAccessToState` _activestate_2 (`local.L_NewStateType`)))
            (:`else`
              _))
          (return))))
    (:`Is Not Valid`
      (goto _label))))

(fn `IsInputPressed`
  (params (InputType :type "/Game/RoadToTemehani/Core/StateManager/EPlayerInputs Enum" :default "NewEnumerator1"))
  (returns (bResult :type Boolean))
  (return (`BlueprintMapLibrary.Map_Find` (`self.CurrentInputsState`) InputType)))

(fn `SelectStateFromBool`
  (params (State_A :type "/Game/RoadToTemehani/Core/StateManager/EPlayerStates Enum" :default "NewEnumerator7") (State_B :type "/Game/RoadToTemehani/Core/StateManager/EPlayerStates Enum" :default "NewEnumerator7") (bSelect_A :type Boolean))
  (`self.HandleStateTransition` (select `bool` bSelect_A :`false` State_B :`true` State_A))
  (return))

(fn `SelectStateFromInputPressed`
  (params (State_A :type "/Game/RoadToTemehani/Core/StateManager/EPlayerStates Enum" :default "NewEnumerator7") (State_B :type "/Game/RoadToTemehani/Core/StateManager/EPlayerStates Enum" :default "NewEnumerator7") (SelectA_IfPressed :type "/Game/RoadToTemehani/Core/StateManager/EPlayerInputs Enum" :default "NewEnumerator1"))
  (`self.SelectStateFromBool` State_A State_B (`self.IsInputPressed` SelectA_IfPressed))
  (return))

(fn `UpdateCurrentInputsState`
  (params (InputType :type "/Game/RoadToTemehani/Core/StateManager/EPlayerInputs Enum" :default "NewEnumerator0") (bPressed :type Boolean))
  (`BlueprintMapLibrary.Map_Add` (`self.CurrentInputsState`) InputType bPressed)
  (return))