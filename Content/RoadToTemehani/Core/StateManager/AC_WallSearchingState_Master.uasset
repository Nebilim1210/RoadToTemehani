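; Master state component for the player state machine that detects walls beside the player in a side-scroller along X.
; Every Update, it line-traces WorldStatic objects right then left, caches the wall's X normal (-1, 0, 1), fires the overridable OnWallFound hook, and clears the value on Exit.
; Child states get helpers to query wall side, test stick input toward the wall, orient the player away from it, and snap the capsule against it.
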(fn `Exit`
  (params (NextState :type "/Game/RoadToTemehani/Core/StateManager/EPlayerStates Enum" :default "NewEnumerator7"))
  (`parent.Exit` NextState)
  (set `self.WallNormalOnX` 0.0)
  (return))

(fn `Find Wall`
  (params (DistanceAlongX :type "Float (double-precision)"))
  (returns (bFoundWall :type Boolean) (`Hit Info` :type "HitResult Structure"))
  (bind _player_actor (`self.Player Actor`))
  (bind _returnvalue (`Actor.K2_GetActorLocation` _player_actor))
  (bind (_outhit _returnvalue_2) (`KismetSystemLibrary.LineTraceSingleForObjects` _returnvalue (+ _returnvalue (`KismetMathLibrary.MakeVector` DistanceAlongX)) (`|MakeArray` "ObjectTypeQuery1" :!type "EObjectTypeQuery Enum") false (`|MakeArray` _player_actor :!type "Actor Object Reference")))
  (return _returnvalue_2 _outhit))

(fn `GetWallOrientation`
  (returns (Result :type "Float (double-precision)"))
  (return (`self.WallNormalOnX`)))

(fn `IsA_WallLeftOfThePlayer`
  (returns (bResult :type Boolean))
  (return (== (`self.WallNormalOnX`) 1.0)))

(fn `IsA_WallRightOfThePlayer`
  (returns (bResult :type Boolean))
  (return (== (`self.WallNormalOnX`) -1.0)))

(fn `IsPlayerCloseToA_Wall`
  (returns (bResult :type Boolean))
  (return (!= (`self.WallNormalOnX`) 0.0)))

(fn `IsPlayerMovingTowardsWall`
  (returns (bResult :type Boolean))
  (return (and (`self.IsPlayerCloseToA_Wall`) (== (+ (`KismetMathLibrary.SignOfFloat` (`/Game/RoadToTemehani/Player/BP_Player.GetMoveRightAxisValue` (`self.Player Actor`))) (`self.WallNormalOnX`)) 0.0))))

(fn `OnWallFound`)

(fn `Orient Player for Wall Movement`
  (if (`self.IsPlayerCloseToA_Wall`)
    (`Actor.K2_SetActorRotation` (`self.Player Actor`) (`KismetMathLibrary.MakeRotator` 0.0 0.0 (`KismetMathLibrary.SelectFloat` 0.0 180.0 (`self.IsA_WallLeftOfThePlayer`))) false))
  (return))

(fn `SnapPlayerToWall`
  (bind _player_actor (`self.Player Actor`))
  (bind (_bfoundwall _hit_info) (`self.Find Wall` (* (`self.WallSearchingDistance`) (`self.GetWallOrientation`) -1.0)))
  (if _bfoundwall
    (`Actor.K2_SetActorLocation` _player_actor (+ (`KismetMathLibrary.MakeVector` (* (`CapsuleComponent.GetScaledCapsuleRadius` (`Character.CapsuleComponent` _player_actor)) (`self.GetWallOrientation`))) (`.Location` (`GameplayStatics.BreakHitResult` _hit_info))) false false)
    (return)
    (else
      (return))))

(fn `Update`
  (`parent.Update`)
  (`self.UpdateWallProximityInfo`) ; Searches permanently if a wall is next to the player or not.
  (return))

(fn `UpdateWallProximityInfo`
  (returns (bWasWallFound :type Boolean))
  (bind _wallsearchingdistance (`self.WallSearchingDistance`))
  (bind _bfoundwall (`self.Find Wall` _wallsearchingdistance))
  (if _bfoundwall
    (set `self.WallNormalOnX` -1.0)
    (else
      (bind _bfoundwall_2 (`self.Find Wall` (* _wallsearchingdistance -1.0)))
      (if _bfoundwall_2
        (set `self.WallNormalOnX` 1.0)
        (else
          (set `self.WallNormalOnX` 0.0)
          (return false)))))
  (`self.OnWallFound`)
  (return true))