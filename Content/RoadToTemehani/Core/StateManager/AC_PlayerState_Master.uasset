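; AC_PlayerState_Master is the base player state for the StateManager, defining the interface that concrete states can override.
; It exposes Enter, Update and Exit lifecycle hooks, plus an OnFailedAccessToState callback, all empty here.
; IsAccessible allows entry by default.
; HandleInput takes an input type and pressed flag and returns whether to change state and to which enum target, defaulting to no change.
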(fn `Enter`
  (params (PreviousState :type "/Game/RoadToTemehani/Core/StateManager/EPlayerStates Enum" :default "NewEnumerator0"))
  (return))

(fn `Exit`
  (params (NextState :type "/Game/RoadToTemehani/Core/StateManager/EPlayerStates Enum" :default "NewEnumerator0"))
  (return))

(fn `HandleInput`
  (params (InputType :type "/Game/RoadToTemehani/Core/StateManager/EPlayerInputs Enum" :default "NewEnumerator0") (bPressed :type Boolean))
  (returns (bChangeState :type Boolean) (TargetState :type "/Game/RoadToTemehani/Core/StateManager/EPlayerStates Enum"))
  (return false "NewEnumerator0"))

(fn `IsAccessible`
  (returns (bResult :type Boolean))
  (return true))

(fn `OnFailedAccessToState`
  (params (TargetState :type "/Game/RoadToTemehani/Core/StateManager/EPlayerStates Enum" :default "NewEnumerator0"))
  (return))

(fn `Update`
  (return))